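; Child dialogue component, apparently a test, scripting the Rapunzel tower conversation where the player guesses a young woman's name in a riddle.
; Dialogue builds a hardcoded German AddDialogue tree: wrong guesses rewind one step, while the correct guess reveals Rapunzel, then sets branch 1 and ends the conversation.
; BeginPlay caches rows from RapunzelturmDT, but only a disconnected draft of the tree reads them, alongside other unused leftover nodes.
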(event `self.ReceiveBeginPlay`
  (`parent.ReceiveBeginPlay`)
  (bind _returnvalue (`|GetDataTableRow` "/Game/Levels/Rapunzelturm/RapunzelturmDT.RapunzelturmDT" "200")
    (:`then`
      (set `self.General` _returnvalue)
      (bind _returnvalue_2 (`|GetDataTableRow` "/Game/Levels/Rapunzelturm/RapunzelturmDT.RapunzelturmDT" "JF")
        (:`then`
          (set `self.JF` _returnvalue_2)
          (bind _returnvalue_3 (`|GetDataTableRow` "/Game/Levels/Rapunzelturm/RapunzelturmDT.RapunzelturmDT" "Dialog0.1")
            (:`then`
              (set `self.01` _returnvalue_3)
              (bind _returnvalue_4 (`|GetDataTableRow` "/Game/Levels/Rapunzelturm/RapunzelturmDT.RapunzelturmDT" "Dialog1.0")
                (:`then`
                  (set `self.10` _returnvalue_4)
                  (bind _returnvalue_5 (`|GetDataTableRow` "/Game/Levels/Rapunzelturm/RapunzelturmDT.RapunzelturmDT" "Dialog1.1")
                    (:`then`
                      (set `self.11` _returnvalue_5)
                      (bind _returnvalue_6 (`|GetDataTableRow` "/Game/Levels/Rapunzelturm/RapunzelturmDT.RapunzelturmDT" "Dialog1.2")
                        (:`then`
                          (set `self.12` _returnvalue_6))))))))))))))

(fn `Dialogue`
  (bind _array (`|MakeArray` "Zurück" :!type "Text"))
  (`parent.Dialogue`)
  (bind (_state _optionindex) (`self.AddDialogue` "Junge Frau" "\"Du weißt ja nich mal, wer ich bin\"" (`|MakeArray` "\"Wetten ich kann es herausfinden\"" :!type "Text")))
  (switch `/Game/Blueprints/DialogSystem/Enum_DialogState` _state
    (:`NewEnumerator0`
      (switch `int` _optionindex
        (:`0`
          (bind (_state_2 _optionindex_2) (`self.AddDialogue` "Junge Frau" "\"Du hältst dich für besonders klug, hm? Wie wäre es mit einem Rätsel?“ \n\"Zwei Lügen eine Wahrheit: Ich bin Schneewittchen, Rapunzel oder Rumpelstilzchen“" (`|MakeArray` "„Du heißt Schneewittchen“" "„Du bist Rumpelstilzchen“" "„Dein Name ist Rapunzel“" :!type "Text")))
          (switch `/Game/Blueprints/DialogSystem/Enum_DialogState` _state_2
            (:`NewEnumerator0`
              (switch `int` _optionindex_2
                (:`0`
                  (bind _state_3 (`self.AddDialogue` "Junge Frau" "\"Pah, die Gute ist an einem Apfel zu Tode erstickt, sehe ich denn tot für dich aus?\"" _array))
                  (switch `/Game/Blueprints/DialogSystem/Enum_DialogState` _state_3
                    (:`NewEnumerator0`
                      (`self.RemoveDialogueProgress` 1 :!label _label)
                      (`self.UpdateSelectedOption` 0))))
                (:`1`
                  (bind _state_4 (`self.AddDialogue` "Junge Frau" "“SOLL DAS EINE BELEIDIGUNG SEIN??”" _array))
                  (switch `/Game/Blueprints/DialogSystem/Enum_DialogState` _state_4
                    (:`NewEnumerator0`
                      (goto _label))))
                (:`2`
                  (bind _state_5 (`self.AddDialogue` "Rapunzel" "“Bist nicht halb so dumm wie erwartet. Wie bist du denn überhaupt hier hochgekommen? Seit je warte ich auf meine Erlösung durch den einen, doch er kam nie! Aus Frust schnitt ich mir die Haare ab. Als ich bemerkte, was ein Scheusal aus mir wurde, konnte ich keinen Tag mehr ruhen.”" (`|MakeArray` "“ich denke du solltest dein Wohl nicht daran messen, wie hübsch du bist. Ich habe viele schöne Gemälde bemerkt, anscheinend macht dich mehr aus als nur meterlanges Haar”" :!type "Text")))
                  (switch `/Game/Blueprints/DialogSystem/Enum_DialogState` _state_5
                    (:`NewEnumerator0`
                      (`self.SetDialogueBranch` 1)
                      (`self.EndConversation`))
                    (:`NewEnumerator1`
                      (`KismetSystemLibrary.PrintString` "updated")
                      (`self.EndConversation`))))))))))))