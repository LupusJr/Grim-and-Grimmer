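; Dialogue child component for the "Fetzen" interaction in the Rapunzelturm level, showing a single dialogue entry.
; On BeginPlay it caches the general row "200" and the "Fetzen" row from the RapunzelturmDT data table.
; The Dialogue override calls the parent, then on tree branch 0 adds the entry with speaker and text from the Fetzen row.
; Its first option ends the conversation; the cached general row is unused here.
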(event `self.ReceiveBeginPlay`
  (`parent.ReceiveBeginPlay`)
  (bind _returnvalue (`|GetDataTableRow` "/Game/Levels/Rapunzelturm/RapunzelturmDT.RapunzelturmDT" "200")
    (:`then`
      (set `self.General` _returnvalue)
      (bind _returnvalue_2 (`|GetDataTableRow` "/Game/Levels/Rapunzelturm/RapunzelturmDT.RapunzelturmDT" "Fetzen")
        (:`then`
          (set `self.Fetzen` _returnvalue_2))))))

(fn `Dialogue`
  (bind (_fetzen_1 _fetzen_2) (break `/Game/Blueprints/DialogSystem/test/AAAAAAAAAAAAAAAAAAAAAAAAAAAAAA` (`self.Fetzen`)))
  (`parent.Dialogue`)
  (switch `int` (`self.ActiveTreeBranch`)
    (:`0`
      (bind (_state _optionindex) (`self.AddDialogue` _fetzen_1 _fetzen_2))
      (switch `/Game/Blueprints/DialogSystem/Enum_DialogState` _state
        (:`NewEnumerator0`
          (switch `int` _optionindex
            (:`0`
              (`self.EndConversation`))))))))