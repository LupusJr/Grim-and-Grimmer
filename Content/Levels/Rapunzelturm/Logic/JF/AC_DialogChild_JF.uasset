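; Dialogue component child that defines all conversations with NPC JF in the Rapunzelturm (Rapunzel tower) level.
; BeginPlay caches text rows from RapunzelturmDT and references to the NPC, curtain and FischDings actors.
; Dialogue switches on ActiveTreeBranch to play fixed lines, random generic lines or nested choice trees, rewinding progress to repeat question menus.
; Certain branches also trigger world events: JF's matchbox (Streichholzschachtel) action and the cloth and mirror-curtain removal.
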(event `self.ReceiveBeginPlay`
  (`parent.ReceiveBeginPlay`)
  (bind _returnvalue (`|GetDataTableRow` "/Game/Levels/Rapunzelturm/RapunzelturmDT.RapunzelturmDT" "200")
    (:`then`
      (set `self.General` _returnvalue)
      (bind _returnvalue_2 (`|GetDataTableRow` "/Game/Levels/Rapunzelturm/RapunzelturmDT.RapunzelturmDT" "JF")
        (:`then`
          (set `self.JF` _returnvalue_2)
          (bind _returnvalue_3 (`|GetDataTableRow` "/Game/Levels/Rapunzelturm/RapunzelturmDT.RapunzelturmDT" "Dialog0.1")
            (:`then`
              (set `self.01` _returnvalue_3)
              (bind _returnvalue_4 (`|GetDataTableRow` "/Game/Levels/Rapunzelturm/RapunzelturmDT.RapunzelturmDT" "Dialog1.0")
                (:`then`
                  (set `self.10` _returnvalue_4)
                  (bind _returnvalue_5 (`|GetDataTableRow` "/Game/Levels/Rapunzelturm/RapunzelturmDT.RapunzelturmDT" "Dialog1.1")
                    (:`then`
                      (set `self.11` _returnvalue_5)
                      (bind _returnvalue_6 (`|GetDataTableRow` "/Game/Levels/Rapunzelturm/RapunzelturmDT.RapunzelturmDT" "Dialog1.2")
                        (:`then`
                          (set `self.12` _returnvalue_6)
                          (bind _returnvalue_7 (`|GetDataTableRow` "/Game/Levels/Rapunzelturm/RapunzelturmDT.RapunzelturmDT" "Dialog1.3")
                            (:`then`
                              (set `self.13` _returnvalue_7)
                              (bind _returnvalue_8 (`|GetDataTableRow` "/Game/Levels/Rapunzelturm/RapunzelturmDT.RapunzelturmDT" "Dialog2")
                                (:`then`
                                  (set `self.2` _returnvalue_8)
                                  (bind _returnvalue_9 (`|GetDataTableRow` "/Game/Levels/Rapunzelturm/RapunzelturmDT.RapunzelturmDT" "Dialog3")
                                    (:`then`
                                      (set `self.3` _returnvalue_9)
                                      (bind _returnvalue_10 (`|GetDataTableRow` "/Game/Levels/Rapunzelturm/RapunzelturmDT.RapunzelturmDT" "Monolog1")
                                        (:`then`
                                          (set `self.Monolog` _returnvalue_10)
                                          (bind _outactors (`GameplayStatics.GetAllActorsOfClass` "/Game/Levels/Rapunzelturm/Logic/JF/NPC_JF.NPC_JF_C"))
                                          (set `self.JF_Ref` (`|GetArrayItem` _outactors))
                                          (bind _outactors_2 (`GameplayStatics.GetAllActorsOfClass` "/Game/Levels/Rapunzelturm/Logic/201-Vorhang+203Spiegel/201-Vorhang.201-Vorhang_C"))
                                          (set `self.Vorhang` (`|GetArrayItem` _outactors_2))
                                          (bind _outactors_3 (`GameplayStatics.GetAllActorsOfClass` "/Game/Levels/Rapunzelturm/Logic/FischDings/FischDings.FischDings_C"))
                                          (set `self.FischDings` (`|GetArrayItem` _outactors_3)))))))))))))))))))))))

(fn `Dialogue`
  (bind (_jf_1 _jf_2 _jf_3 _jf_4 _jf_5 _jf_6) (break `/Game/Blueprints/DialogSystem/test/AAAAAAAAAAAAAAAAAAAAAAAAAAAAAA` (`self.JF`)))
  (bind (_3_1 _3_2 _3_3 _3_4 _3_5 _3_6 _3_7 _3_8 _3_9 _3_10 _3_11 _3_12 _3_13 _3_14 _3_15 _3_16 _3_17 _3_18 _3_19 _3_20 _3_21 _3_22) (break `/Game/Blueprints/DialogSystem/test/AAAAAAAAAAAAAAAAAAAAAAAAAAAAAA` (`self.3`)))
  (bind (_10_1 _10_2 _10_3 _10_4 _10_5 _10_6 _10_7) (break `/Game/Blueprints/DialogSystem/test/AAAAAAAAAAAAAAAAAAAAAAAAAAAAAA` (`self.10`)))
  (bind (_3_1_2 _3_2_2 _3_3_2 _3_4_2 _3_5_2 _3_6_2 _3_7_2) (break `/Game/Blueprints/DialogSystem/test/AAAAAAAAAAAAAAAAAAAAAAAAAAAAAA` (`self.3`)))
  (bind (_3_1_3 _3_2_3 _3_3_3 _3_4_3 _3_5_3 _3_6_3 _3_7_3 _3_8_2) (break `/Game/Blueprints/DialogSystem/test/AAAAAAAAAAAAAAAAAAAAAAAAAAAAAA` (`self.3`)))
  (bind (_3_1_4 _3_2_4 _3_3_4 _3_4_4 _3_5_4 _3_6_4 _3_7_4 _3_8_3 _3_9_2) (break `/Game/Blueprints/DialogSystem/test/AAAAAAAAAAAAAAAAAAAAAAAAAAAAAA` (`self.3`)))
  (bind (_11_1 _11_2) (break `/Game/Blueprints/DialogSystem/test/AAAAAAAAAAAAAAAAAAAAAAAAAAAAAA` (`self.11`)))
  (bind _12_1 (break `/Game/Blueprints/DialogSystem/test/AAAAAAAAAAAAAAAAAAAAAAAAAAAAAA` (`self.12`)))
  (bind (_10_1_2 _10_2_2 _10_3_2 _10_4_2 _10_5_2 _10_6_2) (break `/Game/Blueprints/DialogSystem/test/AAAAAAAAAAAAAAAAAAAAAAAAAAAAAA` (`self.10`)))
  (bind (_11_1_2 _11_2_2) (break `/Game/Blueprints/DialogSystem/test/AAAAAAAAAAAAAAAAAAAAAAAAAAAAAA` (`self.11`)))
  (bind (_12_1_2 _12_2) (break `/Game/Blueprints/DialogSystem/test/AAAAAAAAAAAAAAAAAAAAAAAAAAAAAA` (`self.12`)))
  (bind (_10_1_3 _10_2_3) (break `/Game/Blueprints/DialogSystem/test/AAAAAAAAAAAAAAAAAAAAAAAAAAAAAA` (`self.10`)))
  (bind (_general_1 _general_2 _general_3 _general_4 _general_5 _general_6 _general_7 _general_8 _general_9 _general_10 _general_11 _general_12 _general_13 _general_14 _general_15 _general_16 _general_17 _general_18) (break `/Game/Blueprints/DialogSystem/test/AAAAAAAAAAAAAAAAAAAAAAAAAAAAAA` (`self.General`)))
  (bind (_12_1_3 _12_2_2) (break `/Game/Blueprints/DialogSystem/test/AAAAAAAAAAAAAAAAAAAAAAAAAAAAAA` (`self.12`)))
  (bind (_10_1_4 _10_2_4 _10_3_3 _10_4_3 _10_5_3 _10_6_3 _10_7_2) (break `/Game/Blueprints/DialogSystem/test/AAAAAAAAAAAAAAAAAAAAAAAAAAAAAA` (`self.10`)))
  (bind (_13_1 _13_2 _13_3) (break `/Game/Blueprints/DialogSystem/test/AAAAAAAAAAAAAAAAAAAAAAAAAAAAAA` (`self.13`)))
  (bind (_3_1_5 _3_2_5) (break `/Game/Blueprints/DialogSystem/test/AAAAAAAAAAAAAAAAAAAAAAAAAAAAAA` (`self.3`)))
  (bind (_2_1 _2_2) (break `/Game/Blueprints/DialogSystem/test/AAAAAAAAAAAAAAAAAAAAAAAAAAAAAA` (`self.2`)))
  (bind (_2_1_2 _2_2_2 _2_3) (break `/Game/Blueprints/DialogSystem/test/AAAAAAAAAAAAAAAAAAAAAAAAAAAAAA` (`self.2`)))
  (bind (_2_1_3 _2_2_3 _2_3_2 _2_4) (break `/Game/Blueprints/DialogSystem/test/AAAAAAAAAAAAAAAAAAAAAAAAAAAAAA` (`self.2`)))
  (bind (_2_1_4 _2_2_4 _2_3_3 _2_4_2 _2_5) (break `/Game/Blueprints/DialogSystem/test/AAAAAAAAAAAAAAAAAAAAAAAAAAAAAA` (`self.2`)))
  (bind (_2_1_5 _2_2_5 _2_3_4 _2_4_3 _2_5_2 _2_6) (break `/Game/Blueprints/DialogSystem/test/AAAAAAAAAAAAAAAAAAAAAAAAAAAAAA` (`self.2`)))
  (bind (_monolog_1 _monolog_2) (break `/Game/Blueprints/DialogSystem/test/AAAAAAAAAAAAAAAAAAAAAAAAAAAAAA` (`self.Monolog`)))
  (bind (_3_1_6 _3_2_6 _3_3_5 _3_4_5 _3_5_5 _3_6_5 _3_7_5 _3_8_4 _3_9_3 _3_10_2 _3_11_2 _3_12_2) (break `/Game/Blueprints/DialogSystem/test/AAAAAAAAAAAAAAAAAAAAAAAAAAAAAA` (`self.3`)))
  (bind (_3_1_7 _3_2_7 _3_3_6 _3_4_6 _3_5_6 _3_6_6 _3_7_6 _3_8_5 _3_9_4 _3_10_3 _3_11_3 _3_12_3 _3_13_2 _3_14_2) (break `/Game/Blueprints/DialogSystem/test/AAAAAAAAAAAAAAAAAAAAAAAAAAAAAA` (`self.3`)))
  (bind (_3_1_8 _3_2_8 _3_3_7 _3_4_7 _3_5_7 _3_6_7 _3_7_7 _3_8_6 _3_9_5 _3_10_4 _3_11_4 _3_12_4 _3_13_3 _3_14_3 _3_15_2) (break `/Game/Blueprints/DialogSystem/test/AAAAAAAAAAAAAAAAAAAAAAAAAAAAAA` (`self.3`)))
  (bind (_3_1_9 _3_2_9 _3_3_8 _3_4_8 _3_5_8 _3_6_8 _3_7_8 _3_8_7 _3_9_6 _3_10_5 _3_11_5 _3_12_5 _3_13_4 _3_14_4 _3_15_3 _3_16_2) (break `/Game/Blueprints/DialogSystem/test/AAAAAAAAAAAAAAAAAAAAAAAAAAAAAA` (`self.3`)))
  (bind (_3_1_10 _3_2_10 _3_3_9 _3_4_9 _3_5_9 _3_6_9 _3_7_9 _3_8_8 _3_9_7 _3_10_6 _3_11_6 _3_12_6 _3_13_5 _3_14_5 _3_15_4 _3_16_3 _3_17_2) (break `/Game/Blueprints/DialogSystem/test/AAAAAAAAAAAAAAAAAAAAAAAAAAAAAA` (`self.3`)))
  (bind (_3_1_11 _3_2_11 _3_3_10 _3_4_10 _3_5_10 _3_6_10 _3_7_10 _3_8_9 _3_9_8 _3_10_7 _3_11_7 _3_12_7 _3_13_6 _3_14_6 _3_15_5 _3_16_4 _3_17_3 _3_18_2) (break `/Game/Blueprints/DialogSystem/test/AAAAAAAAAAAAAAAAAAAAAAAAAAAAAA` (`self.3`)))
  (bind (_3_1_12 _3_2_12 _3_3_11 _3_4_11 _3_5_11 _3_6_11 _3_7_11 _3_8_10 _3_9_9 _3_10_8 _3_11_8 _3_12_8 _3_13_7 _3_14_7 _3_15_6 _3_16_5 _3_17_4 _3_18_3 _3_19_2 _3_20_2 _3_21_2) (break `/Game/Blueprints/DialogSystem/test/AAAAAAAAAAAAAAAAAAAAAAAAAAAAAA` (`self.3`)))
  (bind (_01_1 _01_2 _01_3 _01_4 _01_5) (break `/Game/Blueprints/DialogSystem/test/AAAAAAAAAAAAAAAAAAAAAAAAAAAAAA` (`self.01`)))
  (bind (_01_1_2 _01_2_2 _01_3_2 _01_4_2) (break `/Game/Blueprints/DialogSystem/test/AAAAAAAAAAAAAAAAAAAAAAAAAAAAAA` (`self.01`)))
  (bind (_01_1_3 _01_2_3) (break `/Game/Blueprints/DialogSystem/test/AAAAAAAAAAAAAAAAAAAAAAAAAAAAAA` (`self.01`)))
  (bind (_3_1_13 _3_2_13 _3_3_12) (break `/Game/Blueprints/DialogSystem/test/AAAAAAAAAAAAAAAAAAAAAAAAAAAAAA` (`self.3`)))
  (bind (_3_1_14 _3_2_14 _3_3_13 _3_4_12) (break `/Game/Blueprints/DialogSystem/test/AAAAAAAAAAAAAAAAAAAAAAAAAAAAAA` (`self.3`)))
  (`parent.Dialogue`)
  (switch `int` (`self.ActiveTreeBranch`)
    (:`0`
      (bind (_state _optionindex) (`self.AddDialogue` _jf_1 _jf_2))
      (switch `/Game/Blueprints/DialogSystem/Enum_DialogState` _state
        (:`NewEnumerator0`
          (switch `int` _optionindex
            (:`0`
              (`self.EndConversation`))))))
    (:`1`
      (bind (_state_2 _optionindex_2) (`self.AddDialogue` _jf_1 _jf_4))
      (switch `/Game/Blueprints/DialogSystem/Enum_DialogState` _state_2
        (:`NewEnumerator0`
          (switch `int` _optionindex_2
            (:`0`
              (`self.EndConversation`))))))
    (:`2`
      (bind (_state_3 _optionindex_3) (`self.AddDialogue` _jf_1 (select `int` (`KismetMathLibrary.RandomIntegerInRange` 0 7) :`0` _general_3 :`1` _general_4 :`2` _general_5 :`3` _general_6 :`4` _general_7 :`5` _general_8 :`6` _general_9 :`7` _general_10 :`8` _general_11)))
      (switch `/Game/Blueprints/DialogSystem/Enum_DialogState` _state_3
        (:`NewEnumerator0`
          (switch `int` _optionindex_3
            (:`0`
              (`self.EndConversation`))))))
    (:`3`
      (bind (_state_4 _optionindex_4) (`self.AddDialogue` _jf_1 _jf_5))
      (switch `/Game/Blueprints/DialogSystem/Enum_DialogState` _state_4
        (:`NewEnumerator0`
          (switch `int` _optionindex_4
            (:`0`
              (`self.EndConversation`))))))
    (:`4`
      (bind (_state_5 _optionindex_5) (`self.AddDialogue` _jf_1 _jf_6))
      (switch `/Game/Blueprints/DialogSystem/Enum_DialogState` _state_5
        (:`NewEnumerator0`
          (switch `int` _optionindex_5
            (:`0`
              (`self.EndConversation`))))))
    (:`5`
      (bind (_state_6 _optionindex_6) (`self.AddDialogue` "" _01_2_3))
      (switch `/Game/Blueprints/DialogSystem/Enum_DialogState` _state_6
        (:`NewEnumerator0`
          (switch `int` _optionindex_6
            (:`0`
              (bind (_state_7 _optionindex_7) (`self.AddDialogue` _01_1_2 _01_3_2 (`|MakeArray` _01_4_2)))
              (switch `/Game/Blueprints/DialogSystem/Enum_DialogState` _state_7
                (:`NewEnumerator0`
                  (switch `int` _optionindex_7
                    (:`0`
                      (bind (_state_8 _optionindex_8) (`self.AddDialogue` _01_1 _01_5))
                      (switch `/Game/Blueprints/DialogSystem/Enum_DialogState` _state_8
                        (:`NewEnumerator0`
                          (switch `int` _optionindex_8
                            (:`0`
                              (`self.EndConversation`))))))))))))))
    (:`7`
      (bind (_state_9 _optionindex_9) (`self.AddDialogue` "" _10_2_3))
      (switch `/Game/Blueprints/DialogSystem/Enum_DialogState` _state_9
        (:`NewEnumerator0`
          (switch `int` _optionindex_9
            (:`0`
              (bind (_state_10 _optionindex_10) (`self.AddDialogue` _10_1_2 _10_3_2 (`|MakeArray` _10_4_2 _10_5_2 _10_6_2)))
              (switch `/Game/Blueprints/DialogSystem/Enum_DialogState` _state_10
                (:`NewEnumerator0`
                  (switch `int` _optionindex_10
                    (:`0`
                      (bind (_state_11 _optionindex_11) (`self.AddDialogue` _11_1_2 _11_2_2))
                      (switch `/Game/Blueprints/DialogSystem/Enum_DialogState` _state_11
                        (:`NewEnumerator0`
                          (switch `int` _optionindex_11
                            (:`0`
                              (`self.RemoveDialogueProgress` 1)
                              (`self.UpdateSelectedOption` 0))))))
                    (:`1`
                      (bind (_state_12 _optionindex_12) (`self.AddDialogue` _12_1_2 _12_2))
                      (switch `/Game/Blueprints/DialogSystem/Enum_DialogState` _state_12
                        (:`NewEnumerator0`
                          (switch `int` _optionindex_12
                            (:`0`
                              (`self.RemoveDialogueProgress` 1)
                              (`self.UpdateSelectedOption` 0))))))
                    (:`2`
                      (`self.RemoveDialogueProgress` 1)
                      (`self.UpdateSelectedOption` 0)
                      (`self.EndConversation`))))))))))
    (:`8`)
    (:`9`
      (bind (_state_13 _optionindex_13) (`self.AddDialogue` _10_1 _10_3 (`|MakeArray` _10_4 _10_5 _10_6 _10_7)))
      (switch `/Game/Blueprints/DialogSystem/Enum_DialogState` _state_13
        (:`NewEnumerator0`
          (switch `int` _optionindex_13
            (:`0`
              (bind (_state_14 _optionindex_14) (`self.AddDialogue` _11_1 _11_2))
              (switch `/Game/Blueprints/DialogSystem/Enum_DialogState` _state_14
                (:`NewEnumerator0`
                  (switch `int` _optionindex_14
                    (:`0`
                      (`self.RemoveDialogueProgress` 1)
                      (`self.UpdateSelectedOption` 0))))))
            (:`1`
              (bind (_state_15 _optionindex_15) (`self.AddDialogue` _12_1_3 _12_2_2))
              (switch `/Game/Blueprints/DialogSystem/Enum_DialogState` _state_15
                (:`NewEnumerator0`
                  (switch `int` _optionindex_15
                    (:`0`
                      (`self.RemoveDialogueProgress` 1)
                      (`self.UpdateSelectedOption` 0))))))
            (:`2`
              (`self.RemoveDialogueProgress` 1)
              (`self.UpdateSelectedOption` 0))
            (:`3`
              (bind (_state_16 _optionindex_16) (`self.AddDialogue` _12_1 _10_7_2))
              (switch `/Game/Blueprints/DialogSystem/Enum_DialogState` _state_16
                (:`NewEnumerator0`
                  (switch `int` _optionindex_16
                    (:`0`
                      (bind (_state_17 _optionindex_17) (`self.AddDialogue` "" _13_2 (`|MakeArray` _13_3)))
                      (switch `/Game/Blueprints/DialogSystem/Enum_DialogState` _state_17
                        (:`NewEnumerator0`
                          (switch `int` _optionindex_17
                            (:`0`
                              (`self.EndConversation`)
                              (`/Game/Levels/Rapunzelturm/Logic/JF/NPC_JF.Streichholzschachtel` (`self.JF_Ref`)))))))))))))))
    (:`11`
      (bind (_state_18 _optionindex_18) (`self.AddDialogue` "" _2_2))
      (switch `/Game/Blueprints/DialogSystem/Enum_DialogState` _state_18
        (:`NewEnumerator0`
          (switch `int` _optionindex_18
            (:`0`
              (bind (_state_19 _optionindex_19) (`self.AddDialogue` _2_1_2 _2_3))
              (switch `/Game/Blueprints/DialogSystem/Enum_DialogState` _state_19
                (:`NewEnumerator0`
                  (switch `int` _optionindex_19
                    (:`0`
                      (bind (_state_20 _optionindex_20) (`self.AddDialogue` "" _2_4))
                      (switch `/Game/Blueprints/DialogSystem/Enum_DialogState` _state_20
                        (:`NewEnumerator0`
                          (switch `int` _optionindex_20
                            (:`0`
                              (bind (_state_21 _optionindex_21) (`self.AddDialogue` _2_1_4 _2_5))
                              (switch `/Game/Blueprints/DialogSystem/Enum_DialogState` _state_21
                                (:`NewEnumerator0`
                                  (switch `int` _optionindex_21
                                    (:`0`
                                      (bind (_state_22 _optionindex_22) (`self.AddDialogue` "" _2_6))
                                      (switch `/Game/Blueprints/DialogSystem/Enum_DialogState` _state_22
                                        (:`NewEnumerator0`
                                          (switch `int` _optionindex_22
                                            (:`0`
                                              (bind (_state_23 _optionindex_23) (`self.AddDialogue` :`Dialogue` _monolog_2 :`DialogueAudio` "/Game/Levels/Rapunzelturm/Sounds/tuch_fliegt_weg.tuch_fliegt_weg"))
                                              (`/Game/Levels/Rapunzelturm/Logic/FischDings/FischDings.RemoveTuch` (`self.FischDings`))
                                              (`/Game/Levels/Rapunzelturm/Logic/201-Vorhang+203Spiegel/201-Vorhang.VorhangVonSpiegel` (`self.Vorhang`))
                                              (switch `/Game/Blueprints/DialogSystem/Enum_DialogState` _state_23
                                                (:`NewEnumerator0`
                                                  (switch `int` _optionindex_23
                                                    (:`0`
                                                      (`self.EndConversation`)
                                                      (`/Game/Levels/Rapunzelturm/Logic/201-Vorhang+203Spiegel/201-Vorhang.VorhangVonSpiegel` (`self.Vorhang`)))))))))))))))))))))))))))
    (:`13`
      (bind (_state_24 _optionindex_24) (`self.AddDialogue` "" _3_2_5))
      (switch `/Game/Blueprints/DialogSystem/Enum_DialogState` _state_24
        (:`NewEnumerator0`
          (switch `int` _optionindex_24
            (:`0`
              (bind (_state_25 _optionindex_25) (`self.AddDialogue` _3_1_13 _3_3_12))
              (switch `/Game/Blueprints/DialogSystem/Enum_DialogState` _state_25
                (:`NewEnumerator0`
                  (switch `int` _optionindex_25
                    (:`0`
                      (bind (_state_26 _optionindex_26) (`self.AddDialogue` "" _3_4_12))
                      (switch `/Game/Blueprints/DialogSystem/Enum_DialogState` _state_26
                        (:`NewEnumerator0`
                          (switch `int` _optionindex_26
                            (:`0`
                              (bind (_state_27 _optionindex_27) (`self.AddDialogue` _3_1_2 _3_5_2 (`|MakeArray` _3_6_2 _3_7_2)))
                              (switch `/Game/Blueprints/DialogSystem/Enum_DialogState` _state_27
                                (:`NewEnumerator0`
                                  (switch `int` _optionindex_27
                                    (:`0`
                                      _)
                                    (:`1`
                                      _))
                                  (bind (_state_28 _optionindex_28) (`self.AddDialogue` _3_1_3 _3_8_2))
                                  (switch `/Game/Blueprints/DialogSystem/Enum_DialogState` _state_28
                                    (:`NewEnumerator0`
                                      (switch `int` _optionindex_28
                                        (:`0`
                                          (bind (_state_29 _optionindex_29) (`self.AddDialogue` "" _3_9_2))
                                          (switch `/Game/Blueprints/DialogSystem/Enum_DialogState` _state_29
                                            (:`NewEnumerator0`
                                              (switch `int` _optionindex_29
                                                (:`0`
                                                  (bind (_state_30 _optionindex_30) (`self.AddDialogue` _3_1_6 _3_10_2 (`|MakeArray` _3_11_2 _3_12_2)))
                                                  (switch `/Game/Blueprints/DialogSystem/Enum_DialogState` _state_30
                                                    (:`NewEnumerator0`
                                                      (switch `int` _optionindex_30
                                                        (:`0`
                                                          (bind (_state_31 _optionindex_31) (`self.AddDialogue` _3_1_7 _3_14_2))
                                                          (switch `/Game/Blueprints/DialogSystem/Enum_DialogState` _state_31
                                                            (:`NewEnumerator0`
                                                              (switch `int` _optionindex_31
                                                                (:`0`
                                                                  (bind (_state_32 _optionindex_32) (`self.AddDialogue` "" _3_15_2))
                                                                  (switch `/Game/Blueprints/DialogSystem/Enum_DialogState` _state_32
                                                                    (:`NewEnumerator0`
                                                                      (switch `int` _optionindex_32
                                                                        (:`0`
                                                                          (bind (_state_33 _optionindex_33) (`self.AddDialogue` _3_1_9 _3_16_2))
                                                                          (switch `/Game/Blueprints/DialogSystem/Enum_DialogState` _state_33
                                                                            (:`NewEnumerator0`
                                                                              (switch `int` _optionindex_33
                                                                                (:`0`
                                                                                  (bind (_state_34 _optionindex_34) (`self.AddDialogue` _3_1_10 _3_17_2))
                                                                                  (switch `/Game/Blueprints/DialogSystem/Enum_DialogState` _state_34
                                                                                    (:`NewEnumerator0`
                                                                                      (switch `int` _optionindex_34
                                                                                        (:`0`
                                                                                          (bind (_state_35 _optionindex_35) (`self.AddDialogue` "" _3_18_2))
                                                                                          (switch `/Game/Blueprints/DialogSystem/Enum_DialogState` _state_35
                                                                                            (:`NewEnumerator0`
                                                                                              (switch `int` _optionindex_35
                                                                                                (:`0`
                                                                                                  (bind (_state_36 _optionindex_36) (`self.AddDialogue` _3_1_12 _3_19_2 (`|MakeArray` _3_20_2 _3_21_2)))
                                                                                                  (switch `/Game/Blueprints/DialogSystem/Enum_DialogState` _state_36
                                                                                                    (:`NewEnumerator0`
                                                                                                      (switch `int` _optionindex_36
                                                                                                        (:`0`
                                                                                                          (bind (_state_37 _optionindex_37) (`self.AddDialogue` _3_1 _3_22))
                                                                                                          (switch `/Game/Blueprints/DialogSystem/Enum_DialogState` _state_37
                                                                                                            (:`NewEnumerator0`
                                                                                                              (switch `int` _optionindex_37
                                                                                                                (:`0`
                                                                                                                  (`self.EndConversation`))))))))))))))))))))))))))))))))))))))))))))))))))))))))))