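; Dialogue component for the painting (Gemälde) in room R07 of the Rapunzelturm level.
; BeginPlay caches two RapunzelturmDT rows: general lines (200) and the painting's own speaker and line (R07).
; ActiveTreeBranch selects the painting's line, a speaker-only entry, or one of two random pools of general lines; each branch ends the conversation on option 0.
; The first pool's random range never reaches its last line.
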(event `self.ReceiveBeginPlay`
  (`parent.ReceiveBeginPlay`)
  (bind _returnvalue (`|GetDataTableRow` "/Game/Levels/Rapunzelturm/RapunzelturmDT.RapunzelturmDT" "200")
    (:`then`
      (set `self.General` _returnvalue)
      (bind _returnvalue_2 (`|GetDataTableRow` "/Game/Levels/Rapunzelturm/RapunzelturmDT.RapunzelturmDT" "R07")
        (:`then`
          (set `self.Gemälde` _returnvalue_2))))))

(fn `Dialogue`
  (bind (`_gemälde_1` `_gemälde_2`) (break `/Game/Blueprints/DialogSystem/test/AAAAAAAAAAAAAAAAAAAAAAAAAAAAAA` (`self.Gemälde`)))
  (bind (_general_1 _general_2 _general_3 _general_4 _general_5 _general_6 _general_7 _general_8 _general_9 _general_10 _general_11 _general_12 _general_13 _general_14 _general_15 _general_16 _general_17 _general_18) (break `/Game/Blueprints/DialogSystem/test/AAAAAAAAAAAAAAAAAAAAAAAAAAAAAA` (`self.General`)))
  (`parent.Dialogue`)
  (switch `int` (`self.ActiveTreeBranch`)
    (:`0`
      (bind (_state _optionindex) (`self.AddDialogue` `_gemälde_1` `_gemälde_2`))
      (switch `/Game/Blueprints/DialogSystem/Enum_DialogState` _state
        (:`NewEnumerator0`
          (switch `int` _optionindex
            (:`0`
              (`self.EndConversation`))))))
    (:`1`
      (bind (_state_2 _optionindex_2) (`self.AddDialogue` `_gemälde_1` (select `int` (`KismetMathLibrary.RandomIntegerInRange` 0 7) :`0` _general_3 :`1` _general_4 :`2` _general_5 :`3` _general_6 :`4` _general_7 :`5` _general_8 :`6` _general_9 :`7` _general_10 :`8` _general_11)))
      (switch `/Game/Blueprints/DialogSystem/Enum_DialogState` _state_2
        (:`NewEnumerator0`
          (switch `int` _optionindex_2
            (:`0`
              (`self.EndConversation`))))))
    (:`2`
      (bind (_state_3 _optionindex_3) (`self.AddDialogue` `_gemälde_1`))
      (switch `/Game/Blueprints/DialogSystem/Enum_DialogState` _state_3
        (:`NewEnumerator0`
          (switch `int` _optionindex_3
            (:`0`
              (`self.EndConversation`))))))
    (:`3`
      (bind (_state_4 _optionindex_4) (`self.AddDialogue` `_gemälde_1` (select `int` (`KismetMathLibrary.RandomIntegerInRange` 0 6) :`0` _general_12 :`1` _general_13 :`2` _general_14 :`3` _general_15 :`4` _general_16 :`5` _general_17 :`6` _general_18)))
      (switch `/Game/Blueprints/DialogSystem/Enum_DialogState` _state_4
        (:`NewEnumerator0`
          (switch `int` _optionindex_4
            (:`0`
              (`self.EndConversation`))))))))