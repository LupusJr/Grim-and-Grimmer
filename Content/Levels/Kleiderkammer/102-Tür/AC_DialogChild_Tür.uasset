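; Dialogue child component for the door (Tür) in the Kleiderkammer level.
; On BeginPlay it caches two KleiderkammerDT rows: general shared texts and the door's own texts.
; Dialogue picks a line by DialogueTreeIndex: the door's text, one of two random general lines, another general line, or a hardcoded German key-fits unlock message.
; Each branch offers a single option that ends the conversation.
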(event `self.ReceiveBeginPlay`
  (`parent.ReceiveBeginPlay`)
  (bind _returnvalue (`|GetDataTableRow` "/Game/Levels/Kleiderkammer/KleiderkammerDT.KleiderkammerDT" "100")
    (:`then`
      (set `self.General` _returnvalue)
      (bind _returnvalue_2 (`|GetDataTableRow` "/Game/Levels/Kleiderkammer/KleiderkammerDT.KleiderkammerDT" "102")
        (:`then`
          (set `self.Tür` _returnvalue_2))))))

(fn `Dialogue`
  (bind _general_1 (break `/Game/Blueprints/DialogSystem/test/AAAAAAAAAAAAA` (`self.General`)))
  (bind `_tür_1` (break `/Game/Blueprints/DialogSystem/test/AAAAAAAAAAAAA` (`self.Tür`)))
  (bind _general_1_2 (break `/Game/Blueprints/DialogSystem/test/AAAAAAAAAAAAA` (`self.General`)))
  (bind (`_tür_1_2` `_tür_2`) (break `/Game/Blueprints/DialogSystem/test/AAAAAAAAAAAAA` (`self.Tür`)))
  (bind (_general_1_3 _general_2 _general_3 _general_4) (break `/Game/Blueprints/DialogSystem/test/AAAAAAAAAAAAA` (`self.General`)))
  (bind `_tür_1_3` (break `/Game/Blueprints/DialogSystem/test/AAAAAAAAAAAAA` (`self.Tür`)))
  (bind (_general_1_4 _general_2_2 _general_3_2 _general_4_2 _general_5) (break `/Game/Blueprints/DialogSystem/test/AAAAAAAAAAAAA` (`self.General`)))
  (bind `_tür_1_4` (break `/Game/Blueprints/DialogSystem/test/AAAAAAAAAAAAA` (`self.Tür`)))
  (`parent.Dialogue`)
  (switch `int` (`self.DialogueTreeIndex`)
    (:`0`
      (bind (_state _optionindex) (`self.AddDialogue` `_tür_1_2` `_tür_2` (`|MakeArray` _general_1_2)))
      (switch `/Game/Blueprints/DialogSystem/Enum_DialogState` _state
        (:`NewEnumerator0`
          (switch `int` _optionindex
            (:`0`
              (`self.EndConversation`))))))
    (:`1`
      (bind (_state_2 _optionindex_2) (`self.AddDialogue` `_tür_1_3` (select `int` (`KismetMathLibrary.RandomIntegerInRange` 0 1) :`0` _general_3 :`1` _general_4) (`|MakeArray` _general_1_3)))
      (switch `/Game/Blueprints/DialogSystem/Enum_DialogState` _state_2
        (:`NewEnumerator0`
          (switch `int` _optionindex_2
            (:`0`
              (`self.EndConversation`))))))
    (:`2`
      (bind (_state_3 _optionindex_3) (`self.AddDialogue` `_tür_1_4` _general_5 (`|MakeArray` _general_1_4)))
      (switch `/Game/Blueprints/DialogSystem/Enum_DialogState` _state_3
        (:`NewEnumerator0`
          (switch `int` _optionindex_3
            (:`0`
              (`self.EndConversation`))))))
    (:`3`
      (bind (_state_4 _optionindex_4) (`self.AddDialogue` `_tür_1` "„Der Schlüssel passt!\"  \n \n[Du sperrst die Türe auf.]" (`|MakeArray` _general_1)))
      (switch `int` _optionindex_4
        (:`0`
          (`self.EndConversation`))))))