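; Dialog component for the Staffelei (easel) in the Kleiderkammer level, derived from a parent dialog class.
; On BeginPlay it reads the shared General row and the easel's own row from the Kleiderkammer data table.
; The Dialogue function switches on DialogueTreeIndex between three single-line trees, one with easel-specific text and two with general text.
; Each tree offers one general option that ends the conversation.
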(event `self.ReceiveBeginPlay`
  (`parent.ReceiveBeginPlay`)
  (bind _returnvalue (`|GetDataTableRow` "/Game/Levels/Kleiderkammer/KleiderkammerDT.KleiderkammerDT" "100")
    (:`then`
      (set `self.General` _returnvalue)
      (bind _returnvalue_2 (`|GetDataTableRow` "/Game/Levels/Kleiderkammer/KleiderkammerDT.KleiderkammerDT" "107")
        (:`then`
          (set `self.Staffelei` _returnvalue_2))))))

(fn `Dialogue`
  (bind _staffelei_1 (break `/Game/Blueprints/DialogSystem/test/AAAAAAAAAAAAA` (`self.Staffelei`)))
  (bind (_general_1 _general_2) (break `/Game/Blueprints/DialogSystem/test/AAAAAAAAAAAAA` (`self.General`)))
  (bind _general_1_2 (break `/Game/Blueprints/DialogSystem/test/AAAAAAAAAAAAA` (`self.General`)))
  (bind (_staffelei_1_2 _staffelei_2) (break `/Game/Blueprints/DialogSystem/test/AAAAAAAAAAAAA` (`self.Staffelei`)))
  (bind (_general_1_3 _general_2_2 _general_3 _general_4 _general_5) (break `/Game/Blueprints/DialogSystem/test/AAAAAAAAAAAAA` (`self.General`)))
  (bind _staffelei_1_3 (break `/Game/Blueprints/DialogSystem/test/AAAAAAAAAAAAA` (`self.Staffelei`)))
  (`parent.Dialogue`)
  (switch `int` (`self.DialogueTreeIndex`)
    (:`0`
      (bind (_state _optionindex) (`self.AddDialogue` _staffelei_1_2 _staffelei_2 (`|MakeArray` _general_1_2)))
      (switch `/Game/Blueprints/DialogSystem/Enum_DialogState` _state
        (:`NewEnumerator0`
          (switch `int` _optionindex
            (:`0`
              (`self.EndConversation`))))))
    (:`1`
      (bind (_state_2 _optionindex_2) (`self.AddDialogue` _staffelei_1_3 _general_5 (`|MakeArray` _general_1_3)))
      (switch `/Game/Blueprints/DialogSystem/Enum_DialogState` _state_2
        (:`NewEnumerator0`
          (switch `int` _optionindex_2
            (:`0`
              (`self.EndConversation`))))))
    (:`2`
      (bind (_state_3 _optionindex_3) (`self.AddDialogue` _staffelei_1 _general_2 (`|MakeArray` _general_1)))
      (switch `/Game/Blueprints/DialogSystem/Enum_DialogState` _state_3
        (:`NewEnumerator0`
          (switch `int` _optionindex_3
            (:`0`
              (`self.EndConversation`))))))))