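; Dialogue component for the Ratte (rat) NPC in the Kleiderkammer level, derived from a parent dialogue component.
; On BeginPlay it caches the shared General row and the rat's own row from the Kleiderkammer data table.
; Dialogue switches on ActiveTreeBranch to show one rat-specific or shared line, with one branch picking randomly between two shared lines.
; Each branch offers a single option that ends the conversation.
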(event `self.ReceiveBeginPlay`
  (`parent.ReceiveBeginPlay`)
  (bind _returnvalue (`|GetDataTableRow` "/Game/Levels/Kleiderkammer+Rapunzelturm/Kleiderkammer/KleiderkammerDT.KleiderkammerDT" "100")
    (:`then`
      (set `self.General` _returnvalue)
      (bind _returnvalue_2 (`|GetDataTableRow` "/Game/Levels/Kleiderkammer+Rapunzelturm/Kleiderkammer/KleiderkammerDT.KleiderkammerDT" "106")
        (:`then`
          (set `self.Ratte` _returnvalue_2))))))

(fn `Dialogue`
  (bind (_general_1 _general_2 _general_3 _general_4 _general_5) (break `/Game/Blueprints/DialogSystem/test/AAAAAAAAAAAAA` (`self.General`)))
  (bind (_ratte_1 _ratte_2) (break `/Game/Blueprints/DialogSystem/test/AAAAAAAAAAAAA` (`self.Ratte`)))
  (bind _general_1_2 (break `/Game/Blueprints/DialogSystem/test/AAAAAAAAAAAAA` (`self.General`)))
  (bind _ratte_1_2 (break `/Game/Blueprints/DialogSystem/test/AAAAAAAAAAAAA` (`self.Ratte`)))
  (bind _ratte_1_3 (break `/Game/Blueprints/DialogSystem/test/AAAAAAAAAAAAA` (`self.Ratte`)))
  (bind (_general_1_3 _general_2_2 _general_3_2 _general_4_2) (break `/Game/Blueprints/DialogSystem/test/AAAAAAAAAAAAA` (`self.General`)))
  (bind (_ratte_1_4 _ratte_2_2 _ratte_3) (break `/Game/Blueprints/DialogSystem/test/AAAAAAAAAAAAA` (`self.Ratte`)))
  (bind (_general_1_4 _general_2_3 _general_3_3 _general_4_3) (break `/Game/Blueprints/DialogSystem/test/AAAAAAAAAAAAA` (`self.General`)))
  (`parent.Dialogue`)
  (switch `int` (`self.ActiveTreeBranch`)
    (:`0`
      (bind (_state _optionindex) (`self.AddDialogue` _ratte_1 _ratte_2 (`|MakeArray` _general_1_2)))
      (switch `/Game/Blueprints/DialogSystem/Enum_DialogState` _state
        (:`NewEnumerator0`
          (switch `int` _optionindex
            (:`0`
              (`self.EndConversation`))))))
    (:`1`
      (bind (_state_2 _optionindex_2) (`self.AddDialogue` _ratte_1_3 (select `int` (`KismetMathLibrary.RandomIntegerInRange` 0 1) :`0` _general_3_2 :`1` _general_4_2) (`|MakeArray` _general_1_3)))
      (switch `/Game/Blueprints/DialogSystem/Enum_DialogState` _state_2
        (:`NewEnumerator0`
          (switch `int` _optionindex_2
            (:`0`
              (`self.EndConversation`))))))
    (:`2`
      (bind (_state_3 _optionindex_3) (`self.AddDialogue` _ratte_1_4 _ratte_3 (`|MakeArray` _general_1_4)))
      (switch `/Game/Blueprints/DialogSystem/Enum_DialogState` _state_3
        (:`NewEnumerator0`
          (switch `int` _optionindex_3
            (:`0`
              (`self.EndConversation`))))))
    (:`3`
      (bind (_state_4 _optionindex_4) (`self.AddDialogue` _ratte_1_2 _general_5 (`|MakeArray` _general_1)))
      (switch `/Game/Blueprints/DialogSystem/Enum_DialogState` _state_4
        (:`NewEnumerator0`
          (switch `int` _optionindex_4
            (:`0`
              (`self.EndConversation`))))))))