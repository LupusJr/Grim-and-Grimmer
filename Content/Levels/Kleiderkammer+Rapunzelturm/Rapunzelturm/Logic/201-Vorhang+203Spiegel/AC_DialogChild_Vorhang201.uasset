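; Dialogue child component for the curtain (Vorhang 201) in the Rapunzelturm level, supplying its conversation lines.
; On BeginPlay it caches the shared row 200 and the curtain's row 201 from RapunzelturmDT.
; The Dialogue override switches on ActiveTreeBranch to show a curtain-specific or shared line, with one branch picking randomly among four shared lines.
; Each branch is a single line that can end the conversation on pass-through.
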(event `self.ReceiveBeginPlay`
  (`parent.ReceiveBeginPlay`)
  (bind _returnvalue (`|GetDataTableRow` "/Game/Levels/Kleiderkammer+Rapunzelturm/Rapunzelturm/RapunzelturmDT.RapunzelturmDT" "200")
    (:`then`
      (set `self.General` _returnvalue)
      (bind _returnvalue_2 (`|GetDataTableRow` "/Game/Levels/Kleiderkammer+Rapunzelturm/Rapunzelturm/RapunzelturmDT.RapunzelturmDT" "201")
        (:`then`
          (set `self.Vorhang` _returnvalue_2))))))

(fn `Dialogue`
  (bind (_vorhang_1 _vorhang_2 _vorhang_3 _vorhang_4) (break `/Game/Blueprints/DialogSystem/test/AAAAAAAAAAAAAAAAAAAAAAAAAAAAAA` (`self.Vorhang`)))
  (bind (_general_1 _general_2 _general_3 _general_4 _general_5 _general_6 _general_7) (break `/Game/Blueprints/DialogSystem/test/AAAAAAAAAAAAAAAAAAAAAAAAAAAAAA` (`self.General`)))
  (`parent.Dialogue`)
  (switch `int` (`self.ActiveTreeBranch`)
    (:`0`
      (bind (_state _optionindex) (`self.AddDialogue` _vorhang_1 _vorhang_2))
      (switch `/Game/Blueprints/DialogSystem/Enum_DialogState` _state
        (:`NewEnumerator0`
          (switch `int` _optionindex
            (:`0`
              (`self.EndConversation`))))))
    (:`1`
      (bind (_state_2 _optionindex_2) (`self.AddDialogue` _vorhang_1 (select `int` (`KismetMathLibrary.RandomIntegerInRange` 0 3) :`0` _general_3 :`1` _general_4 :`2` _general_5 :`3` _general_6)))
      (switch `/Game/Blueprints/DialogSystem/Enum_DialogState` _state_2
        (:`NewEnumerator0`
          (switch `int` _optionindex_2
            (:`0`
              (`self.EndConversation`))))))
    (:`2`
      (bind (_state_3 _optionindex_3) (`self.AddDialogue` _vorhang_1 _vorhang_4))
      (switch `/Game/Blueprints/DialogSystem/Enum_DialogState` _state_3
        (:`NewEnumerator0`
          (switch `int` _optionindex_3
            (:`0`
              (`self.EndConversation`))))))
    (:`3`
      (bind (_state_4 _optionindex_4) (`self.AddDialogue` _vorhang_1 _general_7))
      (switch `/Game/Blueprints/DialogSystem/Enum_DialogState` _state_4
        (:`NewEnumerator0`
          (switch `int` _optionindex_4
            (:`0`
              (`self.EndConversation`))))))))