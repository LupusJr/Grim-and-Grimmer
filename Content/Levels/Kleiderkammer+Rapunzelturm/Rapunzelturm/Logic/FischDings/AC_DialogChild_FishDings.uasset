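; Dialogue component for the fish object (FischDings) in the Rapunzelturm level, including branches marked Fischmälde and Zettel.
; BeginPlay caches three RapunzelturmDT rows: general lines, FischDings text and F02.
; Dialogue switches on ActiveTreeBranch to show a single entry, either specific text or a random pick from one of two general-line pools.
; Each branch ends the conversation on its first option.
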(event `self.ReceiveBeginPlay`
  (`parent.ReceiveBeginPlay`)
  (bind _returnvalue (`|GetDataTableRow` "/Game/Levels/Kleiderkammer+Rapunzelturm/Rapunzelturm/RapunzelturmDT.RapunzelturmDT" "200")
    (:`then`
      (set `self.General` _returnvalue)
      (bind _returnvalue_2 (`|GetDataTableRow` "/Game/Levels/Kleiderkammer+Rapunzelturm/Rapunzelturm/RapunzelturmDT.RapunzelturmDT" "RB06")
        (:`then`
          (set `self.FischDings` _returnvalue_2)
          (bind _returnvalue_3 (`|GetDataTableRow` "/Game/Levels/Kleiderkammer+Rapunzelturm/Rapunzelturm/RapunzelturmDT.RapunzelturmDT" "F02")
            (:`then`
              (set `self.F02` _returnvalue_3))))))))

(fn `Dialogue`
  (bind (_fischdings_1 _fischdings_2 _fischdings_3 _fischdings_4 _fischdings_5) (break `/Game/Blueprints/DialogSystem/test/AAAAAAAAAAAAAAAAAAAAAAAAAAAAAA` (`self.FischDings`)))
  (bind (_fischdings_1_2 _fischdings_2_2 _fischdings_3_2 _fischdings_4_2 _fischdings_5_2) (break `/Game/Blueprints/DialogSystem/test/AAAAAAAAAAAAAAAAAAAAAAAAAAAAAA` (`self.FischDings`)))
  (bind _f02_1 (break `/Game/Blueprints/DialogSystem/test/AAAAAAAAAAAAAAAAAAAAAAAAAAAAAA` (`self.F02`)))
  (bind (_general_1 _general_2 _general_3 _general_4 _general_5 _general_6 _general_7 _general_8 _general_9 _general_10 _general_11 _general_12 _general_13 _general_14 _general_15 _general_16 _general_17 _general_18) (break `/Game/Blueprints/DialogSystem/test/AAAAAAAAAAAAAAAAAAAAAAAAAAAAAA` (`self.General`)))
  (bind (_general_1_2 _general_2_2 _general_3_2 _general_4_2 _general_5_2 _general_6_2 _general_7_2 _general_8_2 _general_9_2 _general_10_2 _general_11_2 _general_12_2 _general_13_2 _general_14_2 _general_15_2 _general_16_2 _general_17_2 _general_18_2) (break `/Game/Blueprints/DialogSystem/test/AAAAAAAAAAAAAAAAAAAAAAAAAAAAAA` (`self.General`)))
  (bind _returnvalue (select `int` (`KismetMathLibrary.RandomIntegerInRange` 0 7) :`0` _general_3_2 :`1` _general_4_2 :`2` _general_5_2 :`3` _general_6_2 :`4` _general_7_2 :`5` _general_8_2 :`6` _general_9_2 :`7` _general_10_2 :`8` _general_11_2))
  (bind _returnvalue_2 (select `int` (`KismetMathLibrary.RandomIntegerInRange` 0 6) :`0` _general_12_2 :`1` _general_13_2 :`2` _general_14_2 :`3` _general_15_2 :`4` _general_16_2 :`5` _general_17_2 :`6` _general_18_2))
  (`parent.Dialogue`)
  (switch `int` (`self.ActiveTreeBranch`)
    (:`0`
      (bind (_state _optionindex) (`self.AddDialogue` _fischdings_3 _fischdings_4))
      (switch `/Game/Blueprints/DialogSystem/Enum_DialogState` _state
        (:`NewEnumerator0`
          (switch `int` _optionindex
            (:`0`
              (`self.EndConversation`))))))
    (:`1`
      (bind (_state_2 _optionindex_2) (`self.AddDialogue` _fischdings_3 _fischdings_5))
      (switch `/Game/Blueprints/DialogSystem/Enum_DialogState` _state_2
        (:`NewEnumerator0`
          (switch `int` _optionindex_2
            (:`0`
              (`self.EndConversation`))))))
    (:`2`
      (bind (_state_3 _optionindex_3) (`self.AddDialogue` _fischdings_3 _returnvalue))
      (switch `/Game/Blueprints/DialogSystem/Enum_DialogState` _state_3
        (:`NewEnumerator0`
          (switch `int` _optionindex_3
            (:`0`
              (`self.EndConversation`))))))
    (:`3`
      (bind (_state_4 _optionindex_4) (`self.AddDialogue` _fischdings_3 _returnvalue))
      (switch `/Game/Blueprints/DialogSystem/Enum_DialogState` _state_4
        (:`NewEnumerator0`
          (switch `int` _optionindex_4
            (:`0`
              (`self.EndConversation`))))))
    (:`4`
      ;[1 1 1] Fischmälde
      (bind (_state_5 _optionindex_5) (`self.AddDialogue` _fischdings_1_2 _fischdings_2_2))
      (switch `/Game/Blueprints/DialogSystem/Enum_DialogState` _state_5
        (:`NewEnumerator0`
          (switch `int` _optionindex_5
            (:`0`
              (`self.EndConversation`))))))
    (:`5`
      (bind (_state_6 _optionindex_6) (`self.AddDialogue` _fischdings_1_2 _fischdings_5_2))
      (switch `/Game/Blueprints/DialogSystem/Enum_DialogState` _state_6
        (:`NewEnumerator0`
          (switch `int` _optionindex_6
            (:`0`
              (`self.EndConversation`))))))
    (:`6`
      (bind (_state_7 _optionindex_7) (`self.AddDialogue` _fischdings_1_2 _returnvalue_2))
      (switch `/Game/Blueprints/DialogSystem/Enum_DialogState` _state_7
        (:`NewEnumerator0`
          (switch `int` _optionindex_7
            (:`0`
              (`self.EndConversation`))))))
    (:`7`
      ;[1 1 1] Zettel
      (bind (_state_8 _optionindex_8) (`self.AddDialogue` _f02_1))
      (switch `/Game/Blueprints/DialogSystem/Enum_DialogState` _state_8
        (:`NewEnumerator0`
          (switch `int` _optionindex_8
            (:`0`
              (`self.EndConversation`))))))
    (:`8`
      (bind (_state_9 _optionindex_9) (`self.AddDialogue` _f02_1 _fischdings_5_2))
      (switch `/Game/Blueprints/DialogSystem/Enum_DialogState` _state_9
        (:`NewEnumerator0`
          (switch `int` _optionindex_9
            (:`0`
              (`self.EndConversation`))))))
    (:`9`
      (bind (_state_10 _optionindex_10) (`self.AddDialogue` _f02_1 (select `int` (`KismetMathLibrary.RandomIntegerInRange` 0 7) :`0` _general_3 :`1` _general_4 :`2` _general_5 :`3` _general_6 :`4` _general_7 :`5` _general_8 :`6` _general_9 :`7` _general_10 :`8` _general_11)))
      (switch `/Game/Blueprints/DialogSystem/Enum_DialogState` _state_10
        (:`NewEnumerator0`
          (switch `int` _optionindex_10
            (:`0`
              (`self.EndConversation`))))))
    (:`10`
      (bind (_state_11 _optionindex_11) (`self.AddDialogue` _fischdings_3 _returnvalue_2))
      (switch `/Game/Blueprints/DialogSystem/Enum_DialogState` _state_11
        (:`NewEnumerator0`
          (switch `int` _optionindex_11
            (:`0`
              (`self.EndConversation`))))))))