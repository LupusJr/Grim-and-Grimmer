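; Dialogue component for the Rapunzel NPC, holding her German branching conversation.
; Dialogue extends the parent's and switches on ActiveTreeBranch between the main name-guessing riddle and short one-line reactions.
; Wrong guesses rewind dialogue progress, while the right one reveals Rapunzel and leads to branch 1.
; BeginPlay caches the "NPC"-tagged actor owning this component, which receives ConversationClosedMessage on the final riddle node's Updated state.
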(event `self.ReceiveBeginPlay`
  (bind _outactors (`GameplayStatics.GetAllActorsWithTag` "NPC"))
  (for _array_element _outactors
    (`/Engine/EditorBlueprintResources/StandardMacros.IsValid` (`Actor.GetComponentByClass` _array_element "AC_Dialogue_Rapunzel_C")
      (:`Is Valid`
        (set `self.Rapunzel` _array_element)))))

(fn `Dialogue`
  (bind _array (`|MakeArray` "Zurück" :!type "Text"))
  (`parent.Dialogue`)
  (switch `int` (`self.ActiveTreeBranch`)
    (:`0`
      (bind (_state _optionindex) (`self.AddDialogue` "Junge Frau" "\"WAS FÄLLT DIR BLOSS EIN DU KLEINE GÖRE??\" \n  \n[Du hast nun ihre Aufmerksamkeit]" (`|MakeArray` "\"Sie sollten nicht so laut herumschreien, das ist ja schon fast krank\"" :!type "Text")))
      (switch `/Game/Blueprints/DialogSystem/Enum_DialogState` _state
        (:`NewEnumerator0`
          (switch `int` _optionindex
            (:`0`
              (bind (_state_2 _optionindex_2) (`self.AddDialogue` "Junge Frau" "\"KRANK? Der Schmerz in meiner Brust ist gleich einem Dornenbusch, der in meinen Lungen wächst. Jeden Tag wird mir die Luft zum Atmen knapper!\"" (`|MakeArray` "\"Das hört sich ja schön dramatisch an, schwer zu glauben das es jemandem wie Ihnen so schlecht gehen kann\"" :!type "Text")))
              (switch `/Game/Blueprints/DialogSystem/Enum_DialogState` _state_2
                (:`NewEnumerator0`
                  (switch `int` _optionindex_2
                    (:`0`
                      (bind (_state_3 _optionindex_3) (`self.AddDialogue` "Junge Frau" "\"Du weißt ja nich mal, wer ich bin\"" (`|MakeArray` "\"Wetten ich kann es herausfinden\"" :!type "Text")))
                      (switch `/Game/Blueprints/DialogSystem/Enum_DialogState` _state_3
                        (:`NewEnumerator0`
                          (switch `int` _optionindex_3
                            (:`0`
                              (bind (_state_4 _optionindex_4) (`self.AddDialogue` "Junge Frau" "\"Du hältst dich für besonders klug, hm? Wie wäre es mit einem Rätsel?“ \n\"Zwei Lügen eine Wahrheit: Ich bin Schneewittchen, Rapunzel oder Rumpelstilzchen“" (`|MakeArray` "„Du heißt Schneewittchen“" "„Du bist Rumpelstilzchen“" "„Dein Name ist Rapunzel“" :!type "Text")))
                              (switch `/Game/Blueprints/DialogSystem/Enum_DialogState` _state_4
                                (:`NewEnumerator0`
                                  (switch `int` _optionindex_4
                                    (:`0`
                                      (bind _state_5 (`self.AddDialogue` "Junge Frau" "\"Pah, die Gute ist an einem Apfel zu Tode erstickt, sehe ich denn tot für dich aus?\"" _array))
                                      (switch `/Game/Blueprints/DialogSystem/Enum_DialogState` _state_5
                                        (:`NewEnumerator0`
                                          (`self.RemoveDialogueProgress` 1 :!label _label)
                                          (`self.UpdateSelectedOption` 0))))
                                    (:`1`
                                      (bind _state_6 (`self.AddDialogue` "Junge Frau" "“SOLL DAS EINE BELEIDIGUNG SEIN??”" _array))
                                      (switch `/Game/Blueprints/DialogSystem/Enum_DialogState` _state_6
                                        (:`NewEnumerator0`
                                          (goto _label))))
                                    (:`2`
                                      (bind _state_7 (`self.AddDialogue` "Rapunzel" "“Bist nicht halb so dumm wie erwartet. Wie bist du denn überhaupt hier hochgekommen? Seit je warte ich auf meine Erlösung durch den einen, doch er kam nie! Aus Frust schnitt ich mir die Haare ab. Als ich bemerkte, was ein Scheusal aus mir wurde, konnte ich keinen Tag mehr ruhen.”" (`|MakeArray` "“ich denke du solltest dein Wohl nicht daran messen, wie hübsch du bist. Ich habe viele schöne Gemälde bemerkt, anscheinend macht dich mehr aus als nur meterlanges Haar”" :!type "Text")))
                                      (switch `/Game/Blueprints/DialogSystem/Enum_DialogState` _state_7
                                        (:`NewEnumerator0`
                                          (`self.SetDialogueBranch` 1)
                                          (`self.EndConversation`))
                                        (:`NewEnumerator1`
                                          (message `/Game/Blueprints/InteractionSystem/IInteractionInterface.ConversationClosed` (`self.Rapunzel`)))))))))))))))))))))
    (:`1`
      ;[1 1 1] Möglichkeit für andere Dialoge, bei mehrmaligem Ansprechen.
      (bind _state_8 (`self.AddDialogue` "Rapunzel" "" (`|MakeArray` "Es scheint ihr besser zu gehen" :!type "Text")))
      (switch `/Game/Blueprints/DialogSystem/Enum_DialogState` _state_8
        (:`NewEnumerator0`
          (`self.EndConversation`))))
    (:`2`
      (bind _state_9 (`self.AddDialogue` "Junge Frau" " \n  \n[Sie schenkt dir keine Aufmerksamkeit]" (`|MakeArray` "Zurück" :!type "Text")))
      (switch `/Game/Blueprints/DialogSystem/Enum_DialogState` _state_9
        (:`NewEnumerator0`
          (`self.EndConversation`))))
    (:`3`
      (bind _state_10 (`self.AddDialogue` "" " \n  \n[Das kann ich unmöglich nochmal tun]" (`|MakeArray` "Zurück" :!type "Text")))
      (switch `/Game/Blueprints/DialogSystem/Enum_DialogState` _state_10
        (:`NewEnumerator0`
          (`self.EndConversation`))))
    (:`4`
      (bind _state_11 (`self.AddDialogue` "" "\"Danke, das ist sehr nett aber ich habe gerade kein Hunger] \n  \n[Du steckst den Apfel wieder in die Tasche zurück]" (`|MakeArray` "\"Okay\"" :!type "Text")))
      (switch `/Game/Blueprints/DialogSystem/Enum_DialogState` _state_11
        (:`NewEnumerator0`
          (`self.EndConversation`))))
    (:`5`
      (bind _state_12 (`self.AddDialogue` "" " \n  \n[Eine Junge Frau. Sie sieht sehr traurig aus]" (`|MakeArray` "weiter" :!type "Text")))
      (switch `/Game/Blueprints/DialogSystem/Enum_DialogState` _state_12
        (:`NewEnumerator0`
          (`self.EndConversation`))))
    (:`6`
      (bind _state_13 (`self.AddDialogue` "" " \n  \n[Vieleicht würde sie sich über einen Apfel freuen]" (`|MakeArray` "weiter" :!type "Text")))
      (switch `/Game/Blueprints/DialogSystem/Enum_DialogState` _state_13
        (:`NewEnumerator0`
          (`self.EndConversation`))))))