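; Dialogue component for the crate ("Kiste") in the proof-of-concept level, holding German flavour text for examining, kicking and talking to it.
; On BeginPlay it stores a reference to the actor tagged "Kiste" that carries this component.
; Dialogue extends the parent's, selecting a single-option line by DialogueTreeIndex and then ending the conversation.
; Only the kick that springs the lid also sends ConversationClosedMessage to the crate.
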(event `self.ReceiveBeginPlay`
  (bind _outactors (`GameplayStatics.GetAllActorsWithTag` "Kiste"))
  (for _array_element _outactors
    (`/Engine/EditorBlueprintResources/StandardMacros.IsValid` (`Actor.GetComponentByClass` _array_element "AC_Dialog_Kiste_C")
      (:`Is Valid`
        (set `self.Kiste` _array_element)))))

(fn `Dialogue`
  (`parent.Dialogue`)
  (switch `int` (`self.DialogueTreeIndex`)
    (:`0`
      (bind _state (`self.AddDialogue` "" " \n[\"Eine Kiste. Sie scheint verschlossen zu sein\"]" (`|MakeArray` "weiter" :!type "Text")))
      (switch `/Game/Blueprints/DialogSystem/Enum_DialogState` _state
        (:`NewEnumerator0`
          (`self.EndConversation`))))
    (:`1`
      (bind _state_2 (`self.AddDialogue` "" " \n[Du trittst gegen die Kiste. Der Deckel Springt auf. ]" (`|MakeArray` "weiter" :!type "Text")))
      (switch `/Game/Blueprints/DialogSystem/Enum_DialogState` _state_2
        (:`NewEnumerator0`
          (`self.EndConversation`)
          (message `/Game/Blueprints/Inventory/IInteractionInterface.ConversationClosed` (`self.Kiste`)))))
    (:`2`
      (bind _state_3 (`self.AddDialogue` "" "\"O Kiste bitte öffne dich.\" \n[nichts passiert.]" (`|MakeArray` "weiter" :!type "Text")))
      (switch `/Game/Blueprints/DialogSystem/Enum_DialogState` _state_3
        (:`NewEnumerator0`
          (`self.EndConversation`))))
    (:`3`
      (bind _state_4 (`self.AddDialogue` "" "\"Hallo Kiste\"  \n \n\"...\"  \n \n[nichts passiert.]" (`|MakeArray` "weiter" :!type "Text")))
      (switch `/Game/Blueprints/DialogSystem/Enum_DialogState` _state_4
        (:`NewEnumerator0`
          (`self.EndConversation`))))
    (:`4`
      (bind _state_5 (`self.AddDialogue` "" " \n[Du trittst erneut gegen die Kiste. Dein Fuß schmerzt.]" (`|MakeArray` "weiter" :!type "Text")))
      (switch `/Game/Blueprints/DialogSystem/Enum_DialogState` _state_5
        (:`NewEnumerator0`
          (`self.EndConversation`))))))