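; Dialogue component for the curtain (Vorhang) interactable in the proof-of-concept level, giving short German flavour responses when the player interacts with it.
; Overrides Dialogue, calls the parent, then switches on DialogueTreeIndex to choose between wondering what is behind it, kicking it or remarking that it will not answer.
; Each branch is a single AddDialogue line with a continue option that ends the conversation on Pass Through.
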(fn `Dialogue`
  (`parent.Dialogue`)
  (switch `int` (`self.DialogueTreeIndex`)
    (:`0`
      (bind _state (`self.AddDialogue` "" " \n[\"Ich frage mich was sich dahinter verbirgt\"]" (`|MakeArray` "weiter" :!type "Text")))
      (switch `/Game/Blueprints/DialogSystem/Enum_DialogState` _state
        (:`NewEnumerator0`
          (`self.EndConversation`))))
    (:`1`
      (bind _state_2 (`self.AddDialogue` "" " \n[Du trittst gegen den Vorhang. Du hörst ein leises Knacken]" (`|MakeArray` "weiter" :!type "Text")))
      (switch `/Game/Blueprints/DialogSystem/Enum_DialogState` _state_2
        (:`NewEnumerator0`
          (`self.EndConversation`))))
    (:`2`
      (bind _state_3 (`self.AddDialogue` "" " \n[\"Er wird mir nicht antworten\"]" (`|MakeArray` "weiter" :!type "Text")))
      (switch `/Game/Blueprints/DialogSystem/Enum_DialogState` _state_3
        (:`NewEnumerator0`
          (`self.EndConversation`))))))