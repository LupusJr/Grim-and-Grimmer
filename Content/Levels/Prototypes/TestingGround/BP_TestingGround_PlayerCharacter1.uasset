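; Prototype player character for the testing ground level, shown as a 2D Paper2D flipbook.
; Each tick it switches between the idle and walk flipbooks based on whether its velocity is zero.
; It also rotates the flipbook component to face the sign of X velocity, keeping the last facing when X velocity is zero.
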(event `self.ReceiveTick`
  (params (DeltaSeconds :type "Float (single-precision)"))
  (bind _paperflipbook (`self.PaperFlipbook`))
  ;[1 1 1] Flipbook Statemashine
  (`self.SetFlipbookRotation`)
  (if (<= (`KismetMathLibrary.Abs` (`KismetMathLibrary.VSize` (`self.GetVelocity`))) 0.0)
    (`PaperFlipbookComponent.SetFlipbook` _paperflipbook "/Game/Imports/Sprites/Player/Plent/Idle/Idle_Plent.Idle_Plent")
    (else
      (`PaperFlipbookComponent.SetFlipbook` _paperflipbook "/Game/Imports/Sprites/Player/Plent/Walk/Walk_Plent.Walk_Plent"))))

(event `SetFlipbookRotation`
  (bind _paperflipbook (`self.PaperFlipbook`))
  (bind _velocity_x (`KismetMathLibrary.BreakVector` (`MovementComponent.Velocity` (`self.CharacterMovement`))))
  ;[1 1 1] Set Flipbook Rotation
  (`/Engine/EditorBlueprintResources/StandardMacros.CompareFloat` _velocity_x
    (:`>`
      (`SceneComponent.K2_SetRelativeRotation` :`self` _paperflipbook))
    (:`<`
      (`SceneComponent.K2_SetRelativeRotation` _paperflipbook (struct :`Yaw` 180.0) false false))))

(fn `UserConstructionScript`)