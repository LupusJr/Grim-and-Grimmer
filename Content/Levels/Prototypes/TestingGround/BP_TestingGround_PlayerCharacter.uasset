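; BP_TestingGround_PlayerCharacter is a prototype player character that displays a 2D skeleton flipbook in the testing-ground level.
; Each tick it picks the idle or walk flipbook based on whether velocity is zero.
; It also yaws the flipbook component 180 degrees to face the sign of the movement component's X velocity, keeping its last facing when X is zero.
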(event `self.ReceiveTick`
  (params (DeltaSeconds :type "Float (single-precision)"))
  (bind _paperflipbook (`self.PaperFlipbook`))
  ;[1 1 1] Flipbook Statemashine
  (`self.SetFlipbookRotation`)
  (if (<= (`KismetMathLibrary.Abs` (`KismetMathLibrary.VSize` (`self.GetVelocity`))) 0.0)
    (`PaperFlipbookComponent.SetFlipbook` _paperflipbook "/Game/Imports/Sprites/Player/Skeleton/Idle/Idle_Skeleton.Idle_Skeleton")
    (else
      (`PaperFlipbookComponent.SetFlipbook` _paperflipbook "/Game/Imports/Sprites/Player/Skeleton/Walk/Walk_Skeleton.Walk_Skeleton"))))

(event `SetFlipbookRotation`
  (bind _paperflipbook (`self.PaperFlipbook`))
  (bind _velocity_x (`KismetMathLibrary.BreakVector` (`MovementComponent.Velocity` (`self.CharacterMovement`))))
  ;[1 1 1] Set Flipbook Rotation
  (`/Engine/EditorBlueprintResources/StandardMacros.CompareFloat` _velocity_x
    (:`>`
      (`SceneComponent.K2_SetRelativeRotation` _paperflipbook (`KismetMathLibrary.MakeRotator` 0.0) false false))
    (:`<`
      (`SceneComponent.K2_SetRelativeRotation` _paperflipbook (`KismetMathLibrary.MakeRotator` 0.0 0.0 180.0) false false))))

(fn `UserConstructionScript`)