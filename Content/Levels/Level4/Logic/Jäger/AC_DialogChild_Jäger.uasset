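; Dialogue component for the Jäger (hunter) NPC in Level 4, derived from a parent dialogue component.
; BeginPlay caches four rows from the BruderlevelDialog data table in a chain of lookups.
; Dialogue switches on ActiveTreeBranch between single-line replies and two longer conversations with player choices, all of which converge on the same follow-up.
; The longest branch (2) never reaches EndConversation, as its final call is left unconnected.
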(event `self.ReceiveBeginPlay`
  (`parent.ReceiveBeginPlay`)
  (bind _returnvalue (`|GetDataTableRow` "/Game/Blueprints/DialogSystem/test/Bruderlevel-Dialog.Bruderlevel-Dialog" "300")
    (:`then`
      (set `self.300` _returnvalue)
      (bind _returnvalue_2 (`|GetDataTableRow` "/Game/Blueprints/DialogSystem/test/Bruderlevel-Dialog.Bruderlevel-Dialog" "Dialog1")
        (:`then`
          (set `self.Dialog1` _returnvalue_2)
          (bind _returnvalue_3 (`|GetDataTableRow` "/Game/Blueprints/DialogSystem/test/Bruderlevel-Dialog.Bruderlevel-Dialog" "J")
            (:`then`
              (set `self.J` _returnvalue_3)
              (bind _returnvalue_4 (`|GetDataTableRow` "/Game/Blueprints/DialogSystem/test/Bruderlevel-Dialog.Bruderlevel-Dialog" "Dialog2")
                (:`then`
                  (set `self.Dialog2` _returnvalue_4))))))))))

(fn `Dialogue`
  (bind (_dialog1_1 _dialog1_2 _dialog1_3 _dialog1_4 _dialog1_5) (break `/Game/Blueprints/DialogSystem/test/AAAAAAAAAAAAA1` (`self.Dialog1`)))
  (bind (_j_1 _j_2) (break `/Game/Blueprints/DialogSystem/test/AAAAAAAAAAAAA1` (`self.J`)))
  (bind (_dialog2_1 _dialog2_2 _dialog2_3 _dialog2_4 _dialog2_5 _dialog2_6 _dialog2_7 _dialog2_8 _dialog2_9) (break `/Game/Blueprints/DialogSystem/test/AAAAAAAAAAAAA1` (`self.Dialog2`)))
  (bind (_dialog2_1_2 _dialog2_2_2 _dialog2_3_2 _dialog2_4_2 _dialog2_5_2 _dialog2_6_2 _dialog2_7_2 _dialog2_8_2 _dialog2_9_2 _dialog2_10 _dialog2_11 _dialog2_12) (break `/Game/Blueprints/DialogSystem/test/AAAAAAAAAAAAA1` (`self.Dialog2`)))
  (bind (_dialog2_1_3 _dialog2_2_3 _dialog2_3_3 _dialog2_4_3 _dialog2_5_3 _dialog2_6_3 _dialog2_7_3 _dialog2_8_3 _dialog2_9_3 _dialog2_10_2 _dialog2_11_2 _dialog2_12_2 _dialog2_13) (break `/Game/Blueprints/DialogSystem/test/AAAAAAAAAAAAA1` (`self.Dialog2`)))
  (bind (_300_1 _300_2 _300_3 _300_4 _300_5 _300_6) (break `/Game/Blueprints/DialogSystem/test/AAAAAAAAAAAAA1` (`self.300`)))
  (bind _j_1_2 (break `/Game/Blueprints/DialogSystem/test/AAAAAAAAAAAAA1` (`self.J`)))
  (bind (_dialog1_1_2 _dialog1_2_2 _dialog1_3_2 _dialog1_4_2) (break `/Game/Blueprints/DialogSystem/test/AAAAAAAAAAAAA1` (`self.Dialog1`)))
  (bind (_dialog2_1_4 _dialog2_2_4 _dialog2_3_4 _dialog2_4_4 _dialog2_5_4 _dialog2_6_4 _dialog2_7_4 _dialog2_8_4 _dialog2_9_4 _dialog2_10_3 _dialog2_11_3 _dialog2_12_3 _dialog2_13_2 _dialog2_14) (break `/Game/Blueprints/DialogSystem/test/AAAAAAAAAAAAA1` (`self.Dialog2`)))
  (bind (_dialog2_1_5 _dialog2_2_5) (break `/Game/Blueprints/DialogSystem/test/AAAAAAAAAAAAA1` (`self.Dialog2`)))
  (bind (_dialog2_1_6 _dialog2_2_6 _dialog2_3_5 _dialog2_4_5 _dialog2_5_5) (break `/Game/Blueprints/DialogSystem/test/AAAAAAAAAAAAA1` (`self.Dialog2`)))
  (bind (_dialog2_1_7 _dialog2_2_7 _dialog2_3_6 _dialog2_4_6 _dialog2_5_6 _dialog2_6_5) (break `/Game/Blueprints/DialogSystem/test/AAAAAAAAAAAAA1` (`self.Dialog2`)))
  (`parent.Dialogue`)
  (switch `int` (`self.ActiveTreeBranch`)
    (:`0`
      (bind (_state _optionindex) (`self.AddDialogue` _j_1 _j_2))
      (switch `/Game/Blueprints/DialogSystem/Enum_DialogState` _state
        (:`NewEnumerator0`
          (switch `int` _optionindex
            (:`0`
              (`self.EndConversation`))))))
    (:`1`
      (bind (_state_2 _optionindex_2) (`self.AddDialogue` _dialog1_1_2 _dialog1_2_2 (`|MakeArray` _dialog1_3_2 _dialog1_4_2)))
      (switch `/Game/Blueprints/DialogSystem/Enum_DialogState` _state_2
        (:`NewEnumerator0`
          (switch `int` _optionindex_2
            (:`0`
              _)
            (:`1`
              _))
          (bind (_state_3 _optionindex_3) (`self.AddDialogue` _dialog1_1 _dialog1_5))
          (switch `/Game/Blueprints/DialogSystem/Enum_DialogState` _state_3
            (:`NewEnumerator0`
              (switch `int` _optionindex_3
                (:`0`
                  (`self.EndConversation`))))))))
    (:`2`
      (bind (_state_4 _optionindex_4) (`self.AddDialogue` "" _dialog2_2_5))
      (switch `/Game/Blueprints/DialogSystem/Enum_DialogState` _state_4
        (:`NewEnumerator0`
          (switch `int` _optionindex_4
            (:`0`
              (bind (_state_5 _optionindex_5) (`self.AddDialogue` _dialog2_1_6 _dialog2_3_5 (`|MakeArray` _dialog2_4_5 _dialog2_5_5)))
              (switch `/Game/Blueprints/DialogSystem/Enum_DialogState` _state_5
                (:`NewEnumerator0`
                  (switch `int` _optionindex_5
                    (:`0`
                      _)
                    (:`1`
                      _))
                  (bind (_state_6 _optionindex_6) (`self.AddDialogue` _dialog2_1_7 _dialog2_6_5))
                  (switch `/Game/Blueprints/DialogSystem/Enum_DialogState` _state_6
                    (:`NewEnumerator0`
                      (switch `int` _optionindex_6
                        (:`0`
                          (bind (_state_7 _optionindex_7) (`self.AddDialogue` _dialog2_1 _dialog2_7 (`|MakeArray` _dialog2_8 _dialog2_9)))
                          (switch `/Game/Blueprints/DialogSystem/Enum_DialogState` _state_7
                            (:`NewEnumerator0`
                              (switch `int` _optionindex_7
                                (:`0`
                                  _)
                                (:`1`
                                  _))
                              (bind (_state_8 _optionindex_8) (`self.AddDialogue` _dialog2_1_2 _dialog2_10 (`|MakeArray` _dialog2_11 _dialog2_12)))
                              (switch `/Game/Blueprints/DialogSystem/Enum_DialogState` _state_8
                                (:`NewEnumerator0`
                                  (switch `int` _optionindex_8
                                    (:`0`
                                      _)
                                    (:`1`
                                      _))
                                  (bind (_state_9 _optionindex_9) (`self.AddDialogue` _dialog2_1_3 _dialog2_13))
                                  (switch `/Game/Blueprints/DialogSystem/Enum_DialogState` _state_9
                                    (:`NewEnumerator0`
                                      (switch `int` _optionindex_9
                                        (:`0`
                                          (bind (_state_10 _optionindex_10) (`self.AddDialogue` _dialog2_1_4 _dialog2_14))
                                          (switch `/Game/Blueprints/DialogSystem/Enum_DialogState` _state_10
                                            (:`NewEnumerator0`
                                              (switch `int` _optionindex_10))))))))))))))))))))))
    (:`3`
      (bind (_state_11 _optionindex_11) (`self.AddDialogue` _j_1_2 _300_4))
      (switch `/Game/Blueprints/DialogSystem/Enum_DialogState` _state_11
        (:`NewEnumerator0`
          (switch `int` _optionindex_11
            (:`0`
              (`self.EndConversation`))))))
    (:`4`
      (bind (_state_12 _optionindex_12) (`self.AddDialogue` _j_1_2 _300_6))
      (switch `/Game/Blueprints/DialogSystem/Enum_DialogState` _state_12
        (:`NewEnumerator0`
          (switch `int` _optionindex_12
            (:`0`
              (`self.EndConversation`))))))
    (:`5`
      (bind (_state_13 _optionindex_13) (`self.AddDialogue` _j_1_2 _300_3))
      (switch `/Game/Blueprints/DialogSystem/Enum_DialogState` _state_13
        (:`NewEnumerator0`
          (switch `int` _optionindex_13
            (:`0`
              (`self.EndConversation`))))))))