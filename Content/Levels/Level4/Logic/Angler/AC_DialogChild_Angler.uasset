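; Dialogue component for the Angler NPC in Level 4, extending a parent dialogue component with this character's conversations.
; BeginPlay caches four rows from the BruderlevelDialog data table, each lookup chained on the previous one succeeding.
; Dialogue switches on ActiveTreeBranch to play single lines, a scripted exchange or a multi-step choice sequence through AddDialogue.
; Player choices all lead to the same follow-up, and each branch closes with EndConversation.
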(event `self.ReceiveBeginPlay`
  (`parent.ReceiveBeginPlay`)
  (bind _returnvalue (`|GetDataTableRow` "/Game/Blueprints/DialogSystem/test/Bruderlevel-Dialog.Bruderlevel-Dialog" "300")
    (:`then`
      (set `self.300` _returnvalue)
      (bind _returnvalue_2 (`|GetDataTableRow` "/Game/Blueprints/DialogSystem/test/Bruderlevel-Dialog.Bruderlevel-Dialog" "A")
        (:`then`
          (set `self.A` _returnvalue_2)
          (bind _returnvalue_3 (`|GetDataTableRow` "/Game/Blueprints/DialogSystem/test/Bruderlevel-Dialog.Bruderlevel-Dialog" "Dialog3")
            (:`then`
              (set `self.Dialog3` _returnvalue_3)
              (bind _returnvalue_4 (`|GetDataTableRow` "/Game/Blueprints/DialogSystem/test/Bruderlevel-Dialog.Bruderlevel-Dialog" "Dialog4")
                (:`then`
                  (set `self.Dialog4` _returnvalue_4))))))))))

(fn `Dialogue`
  (bind (_300_1 _300_2 _300_3 _300_4 _300_5 _300_6) (break `/Game/Blueprints/DialogSystem/test/AAAAAAAAAAAAA1` (`self.300`)))
  (bind (_dialog3_1 _dialog3_2 _dialog3_3) (break `/Game/Blueprints/DialogSystem/test/AAAAAAAAAAAAA1` (`self.Dialog3`)))
  (bind (_dialog4_1 _dialog4_2) (break `/Game/Blueprints/DialogSystem/test/AAAAAAAAAAAAA1` (`self.Dialog4`)))
  (bind (_dialog4_1_2 _dialog4_2_2 _dialog4_3) (break `/Game/Blueprints/DialogSystem/test/AAAAAAAAAAAAA1` (`self.Dialog4`)))
  (bind (_dialog4_1_3 _dialog4_2_3 _dialog4_3_2 _dialog4_4) (break `/Game/Blueprints/DialogSystem/test/AAAAAAAAAAAAA1` (`self.Dialog4`)))
  (bind (_dialog3_1_2 _dialog3_2_2 _dialog3_3_2 _dialog3_4 _dialog3_5 _dialog3_6 _dialog3_7 _dialog3_8 _dialog3_9 _dialog3_10) (break `/Game/Blueprints/DialogSystem/test/AAAAAAAAAAAAA1` (`self.Dialog3`)))
  (bind (_a_1 _a_2) (break `/Game/Blueprints/DialogSystem/test/AAAAAAAAAAAAA1` (`self.A`)))
  (bind (_dialog3_1_3 _dialog3_2_3 _dialog3_3_3 _dialog3_4_2 _dialog3_5_2 _dialog3_6_2 _dialog3_7_2 _dialog3_8_2 _dialog3_9_2 _dialog3_10_2 _dialog3_11) (break `/Game/Blueprints/DialogSystem/test/AAAAAAAAAAAAA1` (`self.Dialog3`)))
  (bind (_dialog3_1_4 _dialog3_2_4 _dialog3_3_4 _dialog3_4_3 _dialog3_5_3 _dialog3_6_3 _dialog3_7_3 _dialog3_8_3 _dialog3_9_3) (break `/Game/Blueprints/DialogSystem/test/AAAAAAAAAAAAA1` (`self.Dialog3`)))
  (bind (_dialog3_1_5 _dialog3_2_5 _dialog3_3_5 _dialog3_4_4 _dialog3_5_4 _dialog3_6_4 _dialog3_7_4 _dialog3_8_4 _dialog3_9_4 _dialog3_10_3) (break `/Game/Blueprints/DialogSystem/test/AAAAAAAAAAAAA1` (`self.Dialog3`)))
  (bind (_dialog3_1_6 _dialog3_2_6 _dialog3_3_6 _dialog3_4_5 _dialog3_5_5 _dialog3_6_5) (break `/Game/Blueprints/DialogSystem/test/AAAAAAAAAAAAA1` (`self.Dialog3`)))
  (bind (_dialog4_1_4 _dialog4_2_4 _dialog4_3_3 _dialog4_4_2 _dialog4_5) (break `/Game/Blueprints/DialogSystem/test/AAAAAAAAAAAAA1` (`self.Dialog4`)))
  (bind (_dialog4_1_5 _dialog4_2_5 _dialog4_3_4 _dialog4_4_3 _dialog4_5_2 _dialog4_6) (break `/Game/Blueprints/DialogSystem/test/AAAAAAAAAAAAA1` (`self.Dialog4`)))
  (`parent.Dialogue`)
  (switch `int` (`self.ActiveTreeBranch`)
    (:`0`
      (bind (_state _optionindex) (`self.AddDialogue` _a_1 _a_2))
      (switch `/Game/Blueprints/DialogSystem/Enum_DialogState` _state
        (:`NewEnumerator0`
          (switch `int` _optionindex
            (:`0`
              (`self.EndConversation`))))))
    (:`1`
      (bind (_state_2 _optionindex_2) (`self.AddDialogue` _dialog3_1_5 _dialog3_10_3))
      (switch `/Game/Blueprints/DialogSystem/Enum_DialogState` _state_2
        (:`NewEnumerator0`
          (switch `int` _optionindex_2
            (:`0`
              (`self.EndConversation`))))))
    (:`3`
      (bind (_state_3 _optionindex_3) (`self.AddDialogue` "" "" (`|MakeArray` _dialog3_2 _dialog3_3)))
      (switch `/Game/Blueprints/DialogSystem/Enum_DialogState` _state_3
        (:`NewEnumerator0`
          (switch `int` _optionindex_3
            (:`0`
              _)
            (:`1`
              _))
          (bind (_state_4 _optionindex_4) (`self.AddDialogue` _dialog3_1_6 _dialog3_4_5 (`|MakeArray` _dialog3_5_5 _dialog3_6_5)))
          (switch `/Game/Blueprints/DialogSystem/Enum_DialogState` _state_4
            (:`NewEnumerator0`
              (switch `int` _optionindex_4
                (:`0`
                  _)
                (:`1`
                  _))
              (bind (_state_5 _optionindex_5) (`self.AddDialogue` _dialog3_1_4 _dialog3_7_3 (`|MakeArray` _dialog3_8_3 _dialog3_9_3)))
              (switch `/Game/Blueprints/DialogSystem/Enum_DialogState` _state_5
                (:`NewEnumerator0`
                  (switch `int` _optionindex_5
                    (:`0`
                      _)
                    (:`1`
                      _))
                  (bind (_state_6 _optionindex_6) (`self.AddDialogue` _dialog3_1_2 _dialog3_10))
                  (switch `/Game/Blueprints/DialogSystem/Enum_DialogState` _state_6
                    (:`NewEnumerator0`
                      (switch `int` _optionindex_6
                        (:`0`
                          (bind (_state_7 _optionindex_7) (`self.AddDialogue` "" _dialog3_11))
                          (switch `/Game/Blueprints/DialogSystem/Enum_DialogState` _state_7
                            (:`NewEnumerator0`
                              (switch `int` _optionindex_7
                                (:`0`
                                  (`self.EndConversation`))))))))))))))))
    (:`4`
      (bind (_state_8 _optionindex_8) (`self.AddDialogue` _dialog4_1 _dialog4_2))
      (switch `/Game/Blueprints/DialogSystem/Enum_DialogState` _state_8
        (:`NewEnumerator0`
          (switch `int` _optionindex_8
            (:`0`
              (bind (_state_9 _optionindex_9) (`self.AddDialogue` "" _dialog4_3))
              (switch `/Game/Blueprints/DialogSystem/Enum_DialogState` _state_9
                (:`NewEnumerator0`
                  (switch `int` _optionindex_9
                    (:`0`
                      (bind (_state_10 _optionindex_10) (`self.AddDialogue` _dialog4_1_3 _dialog4_4))
                      (switch `/Game/Blueprints/DialogSystem/Enum_DialogState` _state_10
                        (:`NewEnumerator0`
                          (switch `int` _optionindex_10
                            (:`0`
                              (bind (_state_11 _optionindex_11) (`self.AddDialogue` "" _dialog4_5))
                              (switch `/Game/Blueprints/DialogSystem/Enum_DialogState` _state_11
                                (:`NewEnumerator0`
                                  (switch `int` _optionindex_11
                                    (:`0`
                                      (bind (_state_12 _optionindex_12) (`self.AddDialogue` _dialog4_1_5 _dialog4_6))
                                      (switch `/Game/Blueprints/DialogSystem/Enum_DialogState` _state_12
                                        (:`NewEnumerator0`
                                          (switch `int` _optionindex_12
                                            (:`0`
                                              (`self.EndConversation`))))))))))))))))))))))
    (:`6`
      (bind (_state_13 _optionindex_13) (`self.AddDialogue` _a_1 _300_3))
      (switch `/Game/Blueprints/DialogSystem/Enum_DialogState` _state_13
        (:`NewEnumerator0`
          (switch `int` _optionindex_13
            (:`0`
              (`self.EndConversation`))))))
    (:`7`
      (bind (_state_14 _optionindex_14) (`self.AddDialogue` _a_1 _300_4))
      (switch `/Game/Blueprints/DialogSystem/Enum_DialogState` _state_14
        (:`NewEnumerator0`
          (switch `int` _optionindex_14
            (:`0`
              (`self.EndConversation`))))))
    (:`8`
      (bind (_state_15 _optionindex_15) (`self.AddDialogue` _a_1 _300_6))
      (switch `/Game/Blueprints/DialogSystem/Enum_DialogState` _state_15
        (:`NewEnumerator0`
          (switch `int` _optionindex_15
            (:`0`
              (`self.EndConversation`))))))))