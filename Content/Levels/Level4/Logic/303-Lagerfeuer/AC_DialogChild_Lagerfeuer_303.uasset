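; Dialogue child component for the Lagerfeuer (campfire) 303 in Level 4, supplying its single-line conversation branches.
; On BeginPlay it caches three rows from the BruderlevelDialog data table through chained lookups: general (300), 303 and Dialog1.
; The Dialogue override switches on ActiveTreeBranch, showing either the Dialog1 line or one of three General lines.
; Every branch takes its NPC from Dialog1 and ends the conversation on option 0.
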(event `self.ReceiveBeginPlay`
  (`parent.ReceiveBeginPlay`)
  (bind _returnvalue (`|GetDataTableRow` "/Game/Blueprints/DialogSystem/test/Bruderlevel-Dialog.Bruderlevel-Dialog" "300")
    (:`then`
      (set `self.General` _returnvalue)
      (bind _returnvalue_2 (`|GetDataTableRow` "/Game/Blueprints/DialogSystem/test/Bruderlevel-Dialog.Bruderlevel-Dialog" "303")
        (:`then`
          (set `self.303` _returnvalue_2)
          (bind _returnvalue_3 (`|GetDataTableRow` "/Game/Blueprints/DialogSystem/test/Bruderlevel-Dialog.Bruderlevel-Dialog" "Dialog1")
            (:`then`
              (set `self.Dialog1` _returnvalue_3))))))))

(fn `Dialogue`
  (bind (_dialog1_1 _dialog1_2) (break `/Game/Blueprints/DialogSystem/test/AAAAAAAAAAAAA1` (`self.Dialog1`)))
  (bind (_general_1 _general_2 _general_3 _general_4 _general_5 _general_6) (break `/Game/Blueprints/DialogSystem/test/AAAAAAAAAAAAA1` (`self.General`)))
  (`parent.Dialogue`)
  (switch `int` (`self.ActiveTreeBranch`)
    (:`0`
      (bind (_state _optionindex) (`self.AddDialogue` _dialog1_1 _dialog1_2))
      (switch `/Game/Blueprints/DialogSystem/Enum_DialogState` _state
        (:`NewEnumerator0`
          (switch `int` _optionindex
            (:`0`
              (`self.EndConversation`))))))
    (:`1`
      (bind (_state_2 _optionindex_2) (`self.AddDialogue` _dialog1_1 _general_4))
      (switch `/Game/Blueprints/DialogSystem/Enum_DialogState` _state_2
        (:`NewEnumerator0`
          (switch `int` _optionindex_2
            (:`0`
              (`self.EndConversation`))))))
    (:`2`
      (bind (_state_3 _optionindex_3) (`self.AddDialogue` _dialog1_1 _general_6))
      (switch `/Game/Blueprints/DialogSystem/Enum_DialogState` _state_3
        (:`NewEnumerator0`
          (switch `int` _optionindex_3
            (:`0`
              (`self.EndConversation`))))))
    (:`3`
      (bind (_state_4 _optionindex_4) (`self.AddDialogue` _dialog1_1 _general_3))
      (switch `/Game/Blueprints/DialogSystem/Enum_DialogState` _state_4
        (:`NewEnumerator0`
          (switch `int` _optionindex_4
            (:`0`
              (`self.EndConversation`))))))))