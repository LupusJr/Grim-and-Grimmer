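; Dialogue component for the Baum (tree) NPC in Level 4, a child of a shared dialogue parent component.
; BeginPlay caches rows 300 and 304 from the BruderlevelDialog data table.
; The Dialogue override switches on ActiveTreeBranch to show a single line under the row 304 NPC name, taken from row 304 for the first branch and row 300 for the others.
; Each branch ends the conversation on its first option.
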(event `self.ReceiveBeginPlay`
  (`parent.ReceiveBeginPlay`)
  (bind _returnvalue (`|GetDataTableRow` "/Game/Blueprints/DialogSystem/test/Bruderlevel-Dialog.Bruderlevel-Dialog" "300")
    (:`then`
      (set `self.300` _returnvalue)
      (bind _returnvalue_2 (`|GetDataTableRow` "/Game/Blueprints/DialogSystem/test/Bruderlevel-Dialog.Bruderlevel-Dialog" "304")
        (:`then`
          (set `self.304` _returnvalue_2))))))

(fn `Dialogue`
  (bind (_304_1 _304_2) (break `/Game/Blueprints/DialogSystem/test/AAAAAAAAAAAAA1` (`self.304`)))
  (bind (_300_1 _300_2 _300_3 _300_4 _300_5 _300_6) (break `/Game/Blueprints/DialogSystem/test/AAAAAAAAAAAAA1` (`self.300`)))
  (`parent.Dialogue`)
  (switch `int` (`self.ActiveTreeBranch`)
    (:`0`
      (bind (_state _optionindex) (`self.AddDialogue` _304_1 _304_2))
      (switch `/Game/Blueprints/DialogSystem/Enum_DialogState` _state
        (:`NewEnumerator0`
          (switch `int` _optionindex
            (:`0`
              (`self.EndConversation`))))))
    (:`1`
      (bind (_state_2 _optionindex_2) (`self.AddDialogue` _304_1 _300_3))
      (switch `/Game/Blueprints/DialogSystem/Enum_DialogState` _state_2
        (:`NewEnumerator0`
          (switch `int` _optionindex_2
            (:`0`
              (`self.EndConversation`))))))
    (:`2`
      (bind (_state_3 _optionindex_3) (`self.AddDialogue` _304_1 _300_4))
      (switch `/Game/Blueprints/DialogSystem/Enum_DialogState` _state_3
        (:`NewEnumerator0`
          (switch `int` _optionindex_3
            (:`0`
              (`self.EndConversation`))))))
    (:`3`
      (bind (_state_4 _optionindex_4) (`self.AddDialogue` _304_1 _300_6))
      (switch `/Game/Blueprints/DialogSystem/Enum_DialogState` _state_4
        (:`NewEnumerator0`
          (switch `int` _optionindex_4
            (:`0`
              (`self.EndConversation`))))))))