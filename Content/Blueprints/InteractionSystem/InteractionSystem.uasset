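; Interaction system for a point-and-click game that handles cursor hover, context verbs and interaction wheels.
; A per-tick cursor trace sets HoverActor and shows its hover text in a cursor widget; the range check gates nothing.
; Opening a Schwester or Bruder wheel selects the hovered actor.
; German verb events message that actor, while InteractWith prefers its ItemDataComponent and then updates the inventory.
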(event `self.ReceiveBeginPlay`
  ;[1 1 1] Create PnCPlayerController & Inventory System Ref
  (bind _aspn_cplayer_controller (`/Game/Blueprints/BML/BMLActorComponent.BML_PlayerController_Actor` 10.0)
    (:`Sucess`
      (bind _output_get (set `self.PnCPlayerControllerRef` _aspn_cplayer_controller))
      (set `self.InventoryRef` (`Actor.GetComponentByClass` _output_get "/Game/Blueprints/Inventory/InventorySystem.InventorySystem_C"))
      ;[1 1 1] Create Display Message Widget
      (bind _returnvalue (`|CreateWidget` "/Game/Blueprints/Inventory/UI/W_DisplayMessage.W_DisplayMessage_C"))
      (bind _output_get_2 (set `self.DisplayMessage` _returnvalue))
      (`UserWidget.AddToViewport` _output_get_2 0)
      (bind _returnvalue_2 (`|CreateWidget` "/Game/Blueprints/Inventory/UI/W_CursorText.W_CursorText_C"))
      (bind _output_get_3 (set `self.WCursorText` _returnvalue_2))
      (`UserWidget.AddToViewport` _output_get_3 0))))

(event `self.ReceiveTick`
  (params (DeltaSeconds :type "Float (single-precision)"))
  ;[1 1 1] Cast Interaction Trace
  (`self.InteractionTrace`))

(event `Treten`
  ;[1 1 1] IW_Logic
  (message `/Game/Blueprints/InteractionSystem/IInteractionInterface.Treten` (`self.SelectedActor`)))

(event `Enthüllen`
  ;[1 1 1] IW_Logic
  (message `/Game/Blueprints/InteractionSystem/IInteractionInterface.Enthüllen` (`self.SelectedActor`)))

(event `Reden`
  ;[1 1 1] KontextSensitiveInteraction_Logic
  (message `/Game/Blueprints/InteractionSystem/IInteractionInterface.CreateRef` (`self.SelectedActor`) (`self.PnCPlayerControllerRef`)))

(event `Untersuchen`
  ;[1 1 1] KontextSensitiveInteraction_Logic
  (message `/Game/Blueprints/InteractionSystem/IInteractionInterface.Untersuchen` (`self.SelectedActor`)))

(event `Durchschauen`
  ;[1 1 1] IW_Logic
  (message `/Game/Blueprints/InteractionSystem/IInteractionInterface.Durchschauen` (`self.SelectedActor`)))

(event `Interact With`
  (bind _pncplayercontrollerref (`self.PnCPlayerControllerRef`))
  ;[1 1 1] Interact
  (bind _selectedactor (`self.SelectedActor`)
    (:`then`
      (bind _returnvalue (`Actor.GetComponentByClass` _selectedactor "/Game/Blueprints/Inventory/ItemDataComponent.ItemDataComponent_C"))
      (`/Engine/EditorBlueprintResources/StandardMacros.IsValid` _returnvalue
        (:`Is Valid`
          (message `/Game/Blueprints/InteractionSystem/IInteractionInterface.InteractWith` _returnvalue _pncplayercontrollerref))
        (:`Is Not Valid`
          (message `/Game/Blueprints/InteractionSystem/IInteractionInterface.InteractWith` _selectedactor _pncplayercontrollerref)))
      (`/Game/Blueprints/Inventory/InventorySystem.MC_Update` (`self.InventoryRef`)))
    (:`else`)))

(event `AddInterationWheel`
  (params (`Pragmatisch?` :type Boolean :default true))
  (bind _interactionwheelschwester (`self.InteractionWheelSchwester`))
  ;[1 1 1] Show Interaction Wheel
  (`/Engine/EditorBlueprintResources/StandardMacros.IsValid` (`self.HoverActor`)
    (:`Is Valid`
      (`/Engine/EditorBlueprintResources/StandardMacros.IsValid` (`self.InteractionWheelSchwester`)
        (:`Is Valid`
          (`KismetSystemLibrary.PrintString` "iwvalid")
          (if (`Widget.IsVisible` (`self.InteractionWheelSchwester`))
            (`KismetSystemLibrary.PrintString` "removed")
            (`Widget.RemoveFromParent` _interactionwheelschwester)
            (else
              (`UserWidget.AddToViewport` _interactionwheelschwester 0)
              (`self.Set Selected Actor and Create Reference `))))
        (:`Is Not Valid`
          (`KismetSystemLibrary.PrintString` "iwunvalid")
          (if `Pragmatisch?`
            (bind _returnvalue (`|CreateWidget` "/Game/Blueprints/InteractionSystem/WDG_InteractionWheel_Schwester.WDG_InteractionWheel_Schwester_C"))
            (bind _output_get (set `self.InteractionWheelSchwester` _returnvalue))
            (`UserWidget.AddToViewport` _output_get 0)
            (`self.Set Selected Actor and Create Reference `)
            (else
              (bind _returnvalue_2 (`|CreateWidget` "/Game/Blueprints/InteractionSystem/WDG_InteractionWheel_Bruder.WDG_InteractionWheel_Bruder_C"))
              (bind _output_get_2 (set `self.InteractionWheelBruder` _returnvalue_2))
              (`UserWidget.AddToViewport` _output_get_2 0)
              (`self.Set Selected Actor and Create Reference `))))))
    (:`Is Not Valid`
      (`KismetSystemLibrary.PrintString` "hoverunvalid"))))

(event `Set Selected Actor and Create Reference`
  ;[1 1 1] Show Interaction Wheel
  (bind _output_get (set `self.SelectedActor` (`self.HoverActor`)))
  (message `/Game/Blueprints/InteractionSystem/IInteractionInterface.CreateRef` _output_get (`GameplayStatics.GetPlayerController` 0)))

(fn `InteractionTrace`
  (bind _pncplayercontrollerref (`self.PnCPlayerControllerRef`))
  (bind _hoveractor (`self.HoverActor`))
  (bind (_hitresult _returnvalue) (`PlayerController.GetHitResultUnderCursorByChannel` _pncplayercontrollerref "TraceTypeQuery3" true))
  (bind (_bblockinghit _binitialoverlap _time _distance _location _impactpoint _normal _impactnormal _physmat _hitactor) (`GameplayStatics.BreakHitResult` _hitresult))
  (if _returnvalue
    (if (< (`Actor.GetDistanceTo` (`Controller.K2_GetPawn` _pncplayercontrollerref) _hitactor) (`self.Interact Range`))
      _
      (else
        _))
    (if (!= _hitactor (`self.HoverActor`))
      (bind _output_get (set `self.HoverActor` _hitactor))
      (bind _message (message `/Game/Blueprints/InteractionSystem/IInteractionInterface.HoverOver` _output_get))
      (`/Game/Blueprints/Inventory/UI/W_CursorText.ShowMessage` (`self.WCursorText`) _message))
    (else
      (if (`KismetSystemLibrary.IsValid` _hoveractor)
        (bind _output_get_2 (set `self.LastSelectedActor` _hoveractor)))
      (set `self.HoverActor` null)
      (`/Game/Blueprints/Inventory/UI/W_CursorText.ShowMessage` (`self.WCursorText`) ""))))