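; Item data component that lets its owning actor be added to a player's inventory, carrying an item row handle and a quantity.
; BeginPlay turns on replication for the owner.
; The interact event passes the row name and quantity to the inventory system on the interacting PlayerController, then calls InteractWithMessage on the owner if that succeeds.
; HoverOver returns an empty string.
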(event `self.ReceiveBeginPlay`
  ;[1 1 1] Initiate
  (`Actor.SetReplicates` (`self.GetOwner`) true))

(event `/Game/Blueprints/Inventory/IInteractionInterface.InteractWith`
  (params (PlayerController :type "/Game/Blueprints/BPs/PnC_PlayerController Object Reference"))
  (bind _inventorysystemschwester (`/Game/Blueprints/BPs/PnC_PlayerController.InventorySystemSchwester` PlayerController))
  (bind (_itemid_datatable _itemid_rowname) (break `DataTableRowHandle` (`self.ItemID`)))
  ;[1 1 1] Interact with Item
  (`/Engine/EditorBlueprintResources/StandardMacros.IsValid` _inventorysystemschwester
    (:`Is Valid`
      (bind _sucess (`/Game/Blueprints/Inventory/InventorySystem.AddToInventory` _inventorysystemschwester _itemid_rowname (`self.Quantity`)))
      (if _sucess
        (message `/Game/Blueprints/Inventory/IInteractionInterface.InteractWith` (`self.GetOwner`) null)))))

(fn `HoverOver`
  (returns (Message :type Text))
  (return ""))