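; Point-and-click interaction system that lets the player hover over actors and act on them through an interaction wheel.
; Each tick, a cursor trace updates the hovered actor and its on-screen message; the range check currently gates nothing.
; The Interact input stores that actor as selected and toggles the wheel, debounced by a short delay.
; Interact, talk, examine and kick events message the selected actor, with Interact preferring its ItemDataComponent and then updating the inventory.
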(event `self.ReceiveBeginPlay`
  ;[1 1 1] Create PnCPlayerController & Inventory System Ref
  (bind _aspn_cplayer_controller (`/Game/Blueprints/Menu/BML/BMLActorComponent.BMLActorComponent` 10.0)
    (:`Sucess`
      (bind _output_get (set `self.PnCPlayerControllerRef` _aspn_cplayer_controller))
      (set `self.InventoryRef` (`Actor.GetComponentByClass` _output_get "/Game/Blueprints/Inventory/InventorySystem.InventorySystem_C"))
      ;[1 1 1] Create Display Message Widget
      (bind _returnvalue (`|CreateWidget` "/Game/Blueprints/Inventory/UI/W_DisplayMessage.W_DisplayMessage_C"))
      (bind _output_get_2 (set `self.DisplayMessage` _returnvalue))
      (`UserWidget.AddToViewport` _output_get_2 0)
      (bind _returnvalue_2 (`|CreateWidget` "/Game/Blueprints/InteractionSystem/WDG_InteractionWheel.WDG_InteractionWheel_C"))
      (set `self.InteractionWheel` _returnvalue_2))))

(event `self.ReceiveTick`
  (params (DeltaSeconds :type "Float (single-precision)"))
  ;[1 1 1] Cast Interaction Trace
  (`self.InteractionTrace`))

(event `EnhancedInput|/Game/Blueprints/Settings/Actions/Interact`
  (params (ActionValue :type Boolean) (ElapsedSeconds :type "Float (double-precision)") (TriggeredSeconds :type "Float (double-precision)") (InputAction :type "InputAction Object Reference" :default "/Game/Blueprints/Settings/Actions/Interact.Interact"))
  ;[1 1 1] Show Interaction Wheel
  (:`Triggered`
    (`/Engine/EditorBlueprintResources/StandardMacros.IsValid` (`self.HoverActor`)
      (:`Is Valid`
        (`/Engine/EditorBlueprintResources/StandardMacros.DoOnce` false :!label _label
          (:`Completed`
            (`|ExecutionSequence`
              (:`then_0`
                (set `self.SelectedActor` (`self.HoverActor`))
                (bind _interactionwheel (`self.InteractionWheel`)
                  (:`then`
                    (if (`Widget.IsVisible` _interactionwheel)
                      (`Widget.RemoveFromParent` _interactionwheel)
                      (else
                        (`UserWidget.AddToViewport` _interactionwheel 0))))
                  (:`else`)))
              (:`then_1`
                (`KismetSystemLibrary.Delay` 0.2)
                (goto _label :!via `Reset`)))))))))

(event `Interact With`
  (bind _pncplayercontrollerref (`self.PnCPlayerControllerRef`))
  ;[1 1 1] Interact
  (bind _selectedactor (`self.SelectedActor`)
    (:`then`
      (bind _returnvalue (`Actor.GetComponentByClass` _selectedactor "/Game/Blueprints/Inventory/ItemDataComponent.ItemDataComponent_C"))
      (`/Engine/EditorBlueprintResources/StandardMacros.IsValid` _returnvalue
        (:`Is Valid`
          (message `/Game/Blueprints/Inventory/IInteractionInterface.InteractWith` _returnvalue _pncplayercontrollerref))
        (:`Is Not Valid`
          (message `/Game/Blueprints/Inventory/IInteractionInterface.InteractWith` _selectedactor _pncplayercontrollerref)))
      (`/Game/Blueprints/Inventory/InventorySystem.MC_Update` (`self.InventoryRef`)))
    (:`else`)))

(event `Reden`
  (message `/Game/Blueprints/Inventory/IInteractionInterface.Talk` (`self.SelectedActor`) (`self.PnCPlayerControllerRef`)))

(event `Untersuchen`
  (message `/Game/Blueprints/Inventory/IInteractionInterface.Untersuchen` (`self.SelectedActor`)))

(event `Treten`
  (message `/Game/Blueprints/Inventory/IInteractionInterface.Treten` (`self.SelectedActor`)))

(fn `InteractionTrace`
  (bind _pncplayercontrollerref (`self.PnCPlayerControllerRef`))
  (bind _hoveractor (`self.HoverActor`))
  (bind (_hitresult _returnvalue) (`PlayerController.GetHitResultUnderCursorByChannel` _pncplayercontrollerref "TraceTypeQuery3" true))
  (bind (_bblockinghit _binitialoverlap _time _distance _location _impactpoint _normal _impactnormal _physmat _hitactor) (`GameplayStatics.BreakHitResult` _hitresult))
  (if _returnvalue
    (if (< (`Actor.GetDistanceTo` (`Controller.K2_GetPawn` _pncplayercontrollerref) _hitactor) (`self.Interact Range`))
      _
      (else
        _))
    (if (!= _hitactor (`self.HoverActor`))
      (bind _output_get (set `self.HoverActor` _hitactor))
      (bind _message (message `/Game/Blueprints/Inventory/IInteractionInterface.HoverOver` _output_get))
      (`/Game/Blueprints/Inventory/UI/W_DisplayMessage.ShowMessage` (`self.DisplayMessage`) _message))
    (else
      (if (`KismetSystemLibrary.IsValid` _hoveractor)
        (bind _output_get_2 (set `self.LastSelectedActor` _hoveractor)))
      (set `self.HoverActor` null)
      (`/Game/Blueprints/Inventory/UI/W_DisplayMessage.ShowMessage` (`self.DisplayMessage`) ""))))