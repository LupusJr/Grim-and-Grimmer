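; Dialogue component for the Brother NPC, holding joking German/English banter with player-selectable replies.
; The Dialogue override calls its parent, then switches on DialogueTreeIndex between a branching first tree and a one-line second.
; Each AddDialogue's Pass Through state and OptionIndex lead deeper into the branch.
; Endings rewind progress, clear it or switch to the second tree, then end the conversation.
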(fn `Dialogue`
  (`parent.Dialogue`)
  (switch `int` (`self.DialogueTreeIndex`)
    (:`0`
      (bind (_state _optionindex) (`self.AddDialogue` "Brother" "Grim and Grimmer < Revolve Abklatsch " (`|MakeArray` "FRFR" "YESSS" :!type "Text")))
      (switch `/Game/Blueprints/DialogSystem/Enum_DialogState` _state
        (:`NewEnumerator0`
          (switch `int` _optionindex
            (:`0`
              (bind (_state_2 _optionindex_2) (`self.AddDialogue` "Brother" "SCHEIß auf die alle" (`|MakeArray` "aber..." "Wir sind sowieso besser" :!type "Text")))
              (switch `/Game/Blueprints/DialogSystem/Enum_DialogState` _state_2
                (:`NewEnumerator0`
                  (switch `int` _optionindex_2
                    (:`0`
                      (bind (_state_3 _optionindex_3) (`self.AddDialogue` "Brother" "Falsch!! SCHEIß auf die alle!!!" (`|MakeArray` "ok" :!type "Text")))
                      (switch `/Game/Blueprints/DialogSystem/Enum_DialogState` _state_3
                        (:`NewEnumerator0`
                          (switch `int` _optionindex_3
                            (:`0`
                              (`self.RemoveDialogueProgress` 2)
                              (`self.EndConversation`))))))
                    (:`1`
                      (bind _state_4 (`self.AddDialogue` "Brother" "Grim & Grimmer auf die 1!!!!" (`|MakeArray` "Grim & Grimmer auf die 1!!!!" :!type "Text")))
                      (switch `/Game/Blueprints/DialogSystem/Enum_DialogState` _state_4
                        (:`NewEnumerator0`
                          (`self.SetDialogueTreeIndex` 1)
                          (`self.EndConversation`))))))))
            (:`1`
              (bind _state_5 (`self.AddDialogue` "Brother" "Imagine GODOT HAHAHAHAHHAHAHAHAHAHHA" (`|MakeArray` "FR IDIOTS" :!type "Text")))
              (switch `/Game/Blueprints/DialogSystem/Enum_DialogState` _state_5
                (:`NewEnumerator0`
                  (`self.ClearDialogueProgress`)
                  (`self.EndConversation`))))))))
    (:`1`
      (bind _state_6 (`self.AddDialogue` "" "ThreeeNoodles>>>>>>>>>>>>>>>>>>>>" (`|MakeArray` "FR the GREATEST" :!type "Text")))
      (switch `/Game/Blueprints/DialogSystem/Enum_DialogState` _state_6
        (:`NewEnumerator0`
          (`self.ClearDialogueProgress`)
          (`self.EndConversation`))))))