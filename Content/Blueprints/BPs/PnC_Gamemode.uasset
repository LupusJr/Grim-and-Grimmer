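; PnC_Gamemode is a game mode that controls which PlayerStart a player spawns at.
; Its ChoosePlayerStart override gathers all PlayerStart actors in the level and uses the PlayerStart value stored in PnC_GameInstance to select one of the first three.
; An invalid second or third entry falls back to the first.
; Selection relies on the order GetAllActorsOfClass returns, with no tag matching.
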(fn `ChoosePlayerStart`
  (params (Player :type "Controller Object Reference"))
  (returns (ReturnValue :type "Actor Object Reference"))
  (bind _playerstartlist (`self.PlayerStartList`))
  (bind _output (`|GetArrayItem` _playerstartlist 2))
  (bind _output_2 (`|GetArrayItem` _playerstartlist 1))
  (bind _outactors (`GameplayStatics.GetAllActorsOfClass` "/Script/Engine.PlayerStart"))
  (set `self.PlayerStartList` _outactors)
  (bind _aspn_c_game_instance (cast `/Game/Blueprints/BPs/PnC_GameInstance` (`GameplayStatics.GetGameInstance`)))
  (switch `int` (`/Game/Blueprints/BPs/PnC_GameInstance.PlayerStart` _aspn_c_game_instance)
    (:`0`
      _)
    (:`1`
      (`/Engine/EditorBlueprintResources/StandardMacros.IsValid` _output_2
        (:`Is Valid`
          (return _output_2))
        (:`Is Not Valid`
          _)))
    (:`2`
      (`/Engine/EditorBlueprintResources/StandardMacros.IsValid` _output
        (:`Is Valid`
          (return _output))
        (:`Is Not Valid`
          _))))
  (return (`|GetArrayItem` _playerstartlist)))

(fn `UserConstructionScript`)