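; Player controller for point-and-click play, handling click movement, context-sensitive interaction and menu hotkeys.
; On BeginPlay it adds the input mapping, applies saved master and music volumes through a sound mix, and caches the HUD.
; Clicks trace under the cursor, then start dialogue on NPC/Actor-tagged hits in UI-only input, or path there via SimpleMoveToLocation.
; Drag-and-drop re-traces and messages the hit actor, while keys drive the player menu, pause menu and FPS display.
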(event `LoadSettings`
  ;[1 1 1] Load & Apply Settings and Create MainMenu-Widget
  ;[1 1 1] LoadSoundSettings
  (`|ExecutionSequence`
    (:`then_0`
      (bind _returnvalue (`GameplayStatics.LoadGameFromSlot` "SliderValue1"))
      (bind _assave_values (cast `/Game/Blueprints/Savegame/Save_Values` _returnvalue))
      (bind _slidervalue (`/Game/Blueprints/Savegame/Save_Values.SliderValue` _assave_values))
      (`GameplayStatics.SetSoundMixClassOverride` (`self.SoundMixModifier`) "/Engine/EngineSounds/Master.Master" _slidervalue 1.0 0.0)
      (`GameplayStatics.PushSoundMixModifier` (`self.SoundMixModifier`)))
    (:`then_1`
      (bind _returnvalue_2 (`GameplayStatics.LoadGameFromSlot` "SliderValue2"))
      (bind _assave_values_2 (cast `/Game/Blueprints/Savegame/Save_Values` _returnvalue_2))
      (`GameplayStatics.SetSoundMixClassOverride` (`self.SoundMixModifier`) "/Engine/EngineSounds/Music.Music" (* _slidervalue (`/Game/Blueprints/Savegame/Save_Values.SliderValue` _assave_values_2)) 1.0 0.0)
      (`GameplayStatics.PushSoundMixModifier` (`self.SoundMixModifier`)))))

(event `self.ReceiveBeginPlay`
  (bind _returnvalue (subsystem `EnhancedInputLocalPlayerSubsystem`))
  ;[1 1 1] Add Mapping
  (`/Engine/EditorBlueprintResources/StandardMacros.IsValid` _returnvalue
    (:`Is Valid`
      (`EnhancedInputSubsystemInterface.AddMappingContext` _returnvalue "/Game/Blueprints/Settings/Input.Input" 0 (struct))
      ;[1 1 1] Load Settings
      (`self.LoadSettings`)
      ;[1 1 1] Ref to HUD
      (bind _aspn_chud (`/Game/Blueprints/BML/BMLPlayerController.Get_BP_HUD` 10.0)
        (:`Sucess`
          (set `self.HudRef` _aspn_chud))))))

(event `EnhancedInput|/Game/Blueprints/Settings/Actions/SetDestination`
  (params (ActionValue :type Boolean) (ElapsedSeconds :type "Float (double-precision)") (TriggeredSeconds :type "Float (double-precision)") (InputAction :type "InputAction Object Reference" :default "/Game/Blueprints/Settings/Actions/SetDestination.SetDestination"))
  ;[1 1 1] Point and Click Movement
  (:`Started`
    (`self.StopMovement`)
    (`|ExecutionSequence`
      (:`then_0`
        (`self.GetHitActor`))
      (:`then_1`
        (`self.ContextSensitiveInteraction`))))
  (:`Canceled`
    (if (< ElapsedSeconds (`self.ThresholdUntilStart`)) :!label _label
      (`self.MoveTo` (`self.Destination`))))
  (:`Completed`
    (goto _label)))

(event `EnhancedInput|/Game/Blueprints/Settings/Actions/InventoryDown`
  (params (ActionValue :type Boolean) (ElapsedSeconds :type "Float (double-precision)") (TriggeredSeconds :type "Float (double-precision)") (InputAction :type "InputAction Object Reference" :default "/Game/Blueprints/Settings/Actions/InventoryDown.InventoryDown"))
  ;[1 1 1] Toggle Inventory
  (:`Triggered`
    (`/Game/Blueprints/BPs/PnC_HUD.DisplayPlayerMenu` (`self.HudRef`))))

(event `Key|F8`
  (params (Key :type "Key Structure"))
  ;[1 1 1] ShowFPS
  (:`Pressed`
    (`KismetSystemLibrary.ExecuteConsoleCommand` "stat fps" null)))

(event `EnhancedInput|/Game/Blueprints/Settings/Actions/Esc`
  (params (ActionValue :type Boolean) (ElapsedSeconds :type "Float (double-precision)") (TriggeredSeconds :type "Float (double-precision)") (InputAction :type "InputAction Object Reference" :default "/Game/Blueprints/Settings/Actions/Esc.Esc"))
  (bind _hudref (`self.HudRef`))
  ;[1 1 1] Create Pause Menu
  (:`Started`
    (if (not (or (`/Game/Blueprints/BPs/PnC_HUD.MainMenu?` _hudref) (`/Game/Blueprints/BPs/PnC_HUD.OptionsMenu?` _hudref)))
      (if (not (`/Game/Blueprints/BPs/PnC_HUD.PauseMenu?` _hudref))
        (`/Game/Blueprints/BPs/PnC_HUD.Create PauseMenu` (`self.HudRef`))
        (else
          (`Widget.RemoveFromParent` (`/Game/Blueprints/BPs/PnC_HUD.PauseMenu` _hudref))
          (`GameplayStatics.SetGamePaused` false))))))

(event `InputModeUIOnly`
  ;[1 1 1] Handle Input Mode
  (`WidgetBlueprintLibrary.SetInputMode_UIOnlyEx` (`GameplayStatics.GetPlayerController` 0) null))

(event `GetHitActor`
  (bind (_hit _location _hitactor) (`self.GetLocationUnderCursor`))
  ;[1 1 1] ContextSensitiveInteraction
  (if _hit
    (set `self.Hit Actor` _hitactor)
    (set `self.Destination` (`KismetMathLibrary.MakeVector` (.x _location) (.y _location)))))

(event `/Game/Blueprints/InteractionSystem/IInteractionInterface.ConversationClosed`
  ;[1 1 1] Handle Input Mode
  (`WidgetBlueprintLibrary.SetInputMode_GameAndUIEx` (`GameplayStatics.GetPlayerController` 0) null "DoNotLock" false))

(event `ContextSensitiveInteraction`
  (bind _hit_actor (`self.Hit Actor`))
  ;[1 1 1] ContextSensitiveInteraction
  (if (or (`self.ActorHasTag` _hit_actor "NPC") (`self.ActorHasTag` _hit_actor "Actor"))
    (`self.StartDialogue`)
    (else
      (`self.MoveTo` (`self.Destination`)))))

(event `StartDialogue`
  (bind _hit_actor (`self.Hit Actor`))
  ;[1 1 1] ContextSensitiveInteraction
  (message `/Game/Blueprints/InteractionSystem/IInteractionInterface.CreateRef` _hit_actor self)
  (message `/Game/Blueprints/InteractionSystem/IInteractionInterface.Untersuchen` _hit_actor)
  (`self.InputModeUIOnly`))

(event `/Game/Blueprints/InteractionSystem/IInteractionInterface.DragAndDropInteraction`
  (`KismetSystemLibrary.Delay` 0.1)
  (`self.GetHitActor`)
  (message `/Game/Blueprints/InteractionSystem/IInteractionInterface.DragAndDropInteraction` (`self.Hit Actor`)))

(fn `Follow`
  (params (Location :type "Vector Structure"))
  (bind _returnvalue (`self.K2_GetPawn`))
  (`/Engine/EditorBlueprintResources/StandardMacros.IsValid` _returnvalue
    (:`Is Valid`
      (`Pawn.AddMovementInput` _returnvalue (`KismetMathLibrary.GetDirectionUnitVector` (`self.K2_GetActorLocation` _returnvalue) Location) 1.0 false))))

(fn `GetLocationUnderCursor`
  (returns (Hit :type Boolean) (Location :type "Vector Structure") (HitActor :type "Actor Object Reference"))
  (bind (_bblockinghit _binitialoverlap _time _distance _location _impactpoint _normal _impactnormal _physmat _hitactor) (`GameplayStatics.BreakHitResult` (`self.GetHitResultUnderCursorByChannel` "TraceTypeQuery1")))
  (return _bblockinghit _location _hitactor))

(fn `HoverOver`
  (returns (Message :type Text))
  (return ""))

(fn `MoveTo`
  (params (location :type "Vector Structure"))
  (`AIBlueprintHelperLibrary.SimpleMoveToLocation` self location))

(fn `NewFunction`)

(fn `UserConstructionScript`)