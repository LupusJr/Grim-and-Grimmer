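; HUD Blueprint that creates and manages the game's menu, fade-in and inventory widgets.
; BeginPlay pauses the game, opens the main menu and restores the FPS overlay from a saved setting.
; FPS, options and pause events toggle their widgets with flags, while ToggleMainMenu is an empty stub.
; Player and container inventories share one widget reference, with container display alternating through a FlipFlop and requiring that reference to be valid.
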(event `self.ReceiveBeginPlay`
  ;[1 1 1] Create MainMenu on Startup
  (`GameplayStatics.SetGamePaused` true)
  (`self.Create MainMenu`)
  (`self.Load FPSMenu `))

(event `Load FPSMenu`
  ;[1 1 1] Load FPSMenu & Add to Viewport
  (bind _returnvalue (`GameplayStatics.LoadGameFromSlot` "Value2"))
  (bind _assave_values (cast `/Game/Blueprints/Savegame/Save_Values` _returnvalue))
  (if (`/Game/Blueprints/Savegame/Save_Values.IsChecked_Save` _assave_values)
    (set `self.FPSMenu?` true)
    (bind _returnvalue_2 (`|CreateWidget` "/Game/Blueprints/Menu/FPSMenu.FPSMenu_C" (`self.GetOwningPlayerController`)))
    (bind _output_get (set `self.FPSMenu` _returnvalue_2))
    (`UserWidget.AddToViewport` _output_get 1)
    (else
      (set `self.FPSMenu?` false))))

(event `Create FadeInMenu`
  ;[1 1 1] Create FadeIn Widget
  (bind _returnvalue (`|CreateWidget` "/Game/Blueprints/Menu/FadeInMenu.FadeInMenu_C" (`self.GetOwningPlayerController`)))
  (bind _output_get (set `self.FadeInMenu` _returnvalue))
  (`UserWidget.AddToViewport` _output_get 0))

(event `Create CreditsMenu`
  ;[1 1 1] Create CreditsMenu
  (bind _returnvalue (`|CreateWidget` "/Game/Blueprints/Menu/CreditsMenu.CreditsMenu_C" (`self.GetOwningPlayerController`)))
  (bind _output_get (set `self.CreditsMenu` _returnvalue))
  (`UserWidget.AddToViewport` _output_get 0))

(event `Create MainMenu`
  ;[1 1 1] Create MainMenu
  (bind _returnvalue (`|CreateWidget` "/Game/Blueprints/Menu/MainMenu.MainMenu_C" (`self.GetOwningPlayerController`)))
  (bind _output_get (set `self.MainMenu` _returnvalue))
  (`UserWidget.AddToViewport` _output_get 0)
  (set `self.MainMenu?` true)
  (`/Game/Blueprints/Menu/MainMenu.[DEVELOPMENT ONLY]` _output_get))

(event `Create FPSMenu`
  (bind _fpsmenu (`self.FPSMenu`))
  ;[1 1 1] Create FPSMenu
  (if (`self.FPSMenu?`)
    (`/Engine/EditorBlueprintResources/StandardMacros.IsValid` _fpsmenu
      (:`Is Valid`
        (`Widget.RemoveFromParent` _fpsmenu)
        (set `self.FPSMenu?` false)))
    (else
      (bind _returnvalue (`|CreateWidget` "/Game/Blueprints/Menu/FPSMenu.FPSMenu_C" (`self.GetOwningPlayerController`)))
      (bind _output_get (set `self.FPSMenu` _returnvalue))
      (`UserWidget.AddToViewport` _output_get 1)
      (set `self.FPSMenu?` true))))

(event `Create OptionMenu`
  (bind _optionsmenu (`self.OptionsMenu`))
  ;[1 1 1] Create OptionsMenu
  (if (`self.OptionsMenu?`)
    (`/Engine/EditorBlueprintResources/StandardMacros.IsValid` _optionsmenu
      (:`Is Valid`
        (`Widget.RemoveFromParent` _optionsmenu)
        (set `self.OptionsMenu?` false)))
    (else
      (bind _returnvalue (`|CreateWidget` "/Game/Blueprints/Menu/OptionsMenu.OptionsMenu_C" (`self.GetOwningPlayerController`)))
      (bind _output_get (set `self.OptionsMenu` _returnvalue))
      (`UserWidget.AddToViewport` _output_get 0)
      (set `self.OptionsMenu?` true))))

(event `Create PauseMenu`
  (bind _pausemenu (`self.PauseMenu`))
  ;[1 1 1] Create PauseMenu
  (if (`self.PauseMenu?`)
    (`/Engine/EditorBlueprintResources/StandardMacros.IsValid` _pausemenu
      (:`Is Valid`
        (`Widget.RemoveFromParent` _pausemenu)
        (set `self.PauseMenu?` false)))
    (else
      (bind _returnvalue (`|CreateWidget` "/Game/Blueprints/Menu/PauseMenu.PauseMenu_C" (`self.GetOwningPlayerController`)))
      (bind _output_get (set `self.PauseMenu` _returnvalue))
      (`UserWidget.AddToViewport` _output_get 0)
      (set `self.PauseMenu?` true))))

(event `ToggleMainMenu`
  ;[1 1 1] Toggle MainMenu
)

(event `DisplayPlayerMenu`
  (bind _playermenu (`self.PlayerMenu`))
  ;[1 1 1] Display Inventory
  (`/Engine/EditorBlueprintResources/StandardMacros.IsValid` _playermenu
    (:`Is Valid`
      (if (not (`Widget.IsInViewport` _playermenu))
        (bind _returnvalue (`|CreateWidget` "/Game/Blueprints/Inventory/UI/W_PlayerMenu.W_PlayerMenu_C" :!label _label))
        (bind _output_get (set `self.PlayerMenu` _returnvalue))
        (`UserWidget.AddToViewport` _output_get 0)))
    (:`Is Not Valid`
      (goto _label))))

(event `ShowContainer`
  (params (ContainerInventory :type "/Game/Blueprints/Inventory/InventorySystem Object Reference"))
  (bind _playermenu (`self.PlayerMenu`))
  ;[1 1 1] Display Container (chest) Inventory
  (`/Engine/EditorBlueprintResources/StandardMacros.IsValid` _playermenu
    (:`Is Valid`
      (if (not (not (`Widget.IsInViewport` _playermenu)))
        (`Widget.RemoveFromParent` _playermenu))
      (`/Engine/EditorBlueprintResources/StandardMacros.FlipFlop`
        (:`A`
          (bind _returnvalue (`|CreateWidget` "/Game/Blueprints/Inventory/UI/W_ContainerInventory.W_ContainerInventory_C" null ContainerInventory))
          (bind _output_get (set `self.PlayerMenu` _returnvalue))
          (`UserWidget.AddToViewport` _output_get 0))
        (:`B`
          (`Widget.RemoveFromParent` _playermenu))))))

(fn `UserConstructionScript`)