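; Game instance for the point-and-click game, handling startup, music, screen fades and story flags that persist across levels.
; Init applies user settings, restores Master and Music volumes from save slots (Music scaled by Master), resets saved door and visibility flags, then pauses the game.
; Helper functions crossfade the active theme and spawn FadeMenu widgets for menu and level transitions.
; Simple events set progress flags such as RatteTod and WolfErwecken.
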(event `self.ReceiveInit`
  (`|ExecutionSequence`
    (:`then_0`
      (bind _returnvalue (`GameUserSettings.GetGameUserSettings`))
      (`GameUserSettings.LoadSettings` _returnvalue false)
      (`GameUserSettings.ApplySettings` _returnvalue true)
      (`GameUserSettings.ApplyResolutionSettings` _returnvalue false)
      (`|ExecutionSequence`
        (:`then_0`
          (bind _returnvalue_2 (`GameplayStatics.LoadGameFromSlot` "SliderValue1"))
          (bind _assave_values (cast `/Game/Blueprints/Savegame/Save_Values` _returnvalue_2))
          (bind _slidervalue (`/Game/Blueprints/Savegame/Save_Values.SliderValue` _assave_values))
          (`GameplayStatics.SetSoundMixClassOverride` (`self.SoundMixModifier`) "/Engine/EngineSounds/Master.Master" _slidervalue 1.0 0.0)
          (`GameplayStatics.PushSoundMixModifier` (`self.SoundMixModifier`)))
        (:`then_1`
          (bind _returnvalue_3 (`GameplayStatics.LoadGameFromSlot` "SliderValue2"))
          (bind _assave_values_2 (cast `/Game/Blueprints/Savegame/Save_Values` _returnvalue_3))
          (`GameplayStatics.SetSoundMixClassOverride` (`self.SoundMixModifier`) "/Engine/EngineSounds/Music.Music" (* _slidervalue (`/Game/Blueprints/Savegame/Save_Values.SliderValue` _assave_values_2)) 1.0 0.0)
          (`GameplayStatics.PushSoundMixModifier` (`self.SoundMixModifier`)))))
    (:`then_1`
      (bind _returnvalue_4 (`GameplayStatics.LoadGameFromSlot` "OULR"))
      (bind _assave_values_3 (cast `/Game/Blueprints/Savegame/Save_Values` _returnvalue_4))
      (set `/Game/Blueprints/Savegame/Save_Values.IsVisibleOL` false _assave_values_3)
      (set `/Game/Blueprints/Savegame/Save_Values.IsVisibleOR` false _assave_values_3)
      (set `/Game/Blueprints/Savegame/Save_Values.IsVisibleUL` false _assave_values_3)
      (set `/Game/Blueprints/Savegame/Save_Values.IsVisibleUR` false _assave_values_3)
      (`GameplayStatics.SaveGameToSlot` _assave_values_3 "OULR"))
    (:`then_2`
      (bind _returnvalue_5 (`GameplayStatics.LoadGameFromSlot` "Tür"))
      (bind _assave_values_4 (cast `/Game/Blueprints/Savegame/Save_Values` _returnvalue_5))
      (set `/Game/Blueprints/Savegame/Save_Values.TürOffen?` false _assave_values_4)
      (`GameplayStatics.SaveGameToSlot` _assave_values_4 "Tür"))
    (:`then_3`
      (bind _output_get (set `self.RatteTod?` false)))
    (:`then_4`
      (`GameplayStatics.SetGamePaused` true)
      (`KismetSystemLibrary.Delay` 0.05))))

(event `MainMenu`
  (bind _returnvalue (`|CreateWidget` "/Game/Blueprints/Menu/FadeMenu.FadeMenu_C"))
  (bind _output_get (set `self.FadeInMenu` _returnvalue))
  (`UserWidget.AddToViewport` _output_get 6)
  (`/Game/Blueprints/Menu/FadeMenu.FadeIn3` (`self.FadeInMenu`))
  (`self.SwitchMusic` 3.0 "/Game/Imports/Awwee/MainTheme.MainTheme")
  (bind _returnvalue_2 (`|CreateWidget` "/Game/Blueprints/Menu/MainMenu.MainMenu_C"))
  (`UserWidget.AddToViewport` _returnvalue_2 3))

(event `FadeOut3Sec`
  (bind _fadeinmenu (`self.FadeOut` 3.0))
  (`/Game/Blueprints/Menu/FadeMenu.FadeOut3` _fadeinmenu))

(event `FadeOutWithoutMusic2Sec`
  (bind _returnvalue (`|CreateWidget` "/Game/Blueprints/Menu/FadeMenu.FadeMenu_C"))
  (bind _output_get (set `self.FadeInMenu` _returnvalue))
  (`UserWidget.AddToViewport` _output_get 6)
  (`/Game/Blueprints/Menu/FadeMenu.FadeOut2` (`self.FadeInMenu`)))

(event `FadeInLevel1`
  (bind _fadeinmenu (`self.FadeIn` "/Game/Levels/Rapunzelturm/Sounds/Schwester_ThemeWav.Schwester_ThemeWav" 3.0))
  (`/Game/Blueprints/Menu/FadeMenu.FadeIn3` _fadeinmenu))

(event `RemoveTuch`
  (set `self.TuchWeg?` true))

(event `JägerWeg`
  (set `self.JägerGone` true))

(event `FadeOut2Sec`
  (bind _fadeinmenu (`self.FadeOut` 2.0))
  (`/Game/Blueprints/Menu/FadeMenu.FadeOut2` _fadeinmenu))

(event `WolfErwecken!`
  (set `self.WolfErwecken?` true))

(event `FadeIn2Sec`
  (bind _returnvalue (`|CreateWidget` "/Game/Blueprints/Menu/FadeMenu.FadeMenu_C"))
  (bind _output_get (set `self.FadeInMenu` _returnvalue))
  (`UserWidget.AddToViewport` _output_get 6)
  (`/Game/Blueprints/Menu/FadeMenu.FadeIn2` (`self.FadeInMenu`)))

(event `RatteTod`
  (set `self.RatteTod?` true))

(event `MotteWeg`
  (set `self.MotteWeg?` true))

(event `SetHigh`
  (bind _aspn_c_player_controller (cast `/Game/Blueprints/BPs/PnC_PlayerController` (`GameplayStatics.GetPlayerController` 0)))
  (set `self.HighInst` (`/Game/Blueprints/BPs/PnC_PlayerController.High` _aspn_c_player_controller)))

(fn `FadeIn`
  (params (Sound :type "SoundBase Object Reference") (FadeInDuration :type "Float (single-precision)"))
  (returns (FadeInMenu :type "/Game/Blueprints/Menu/FadeMenu Object Reference"))
  (bind _returnvalue (`GameplayStatics.CreateSound2D` Sound 1.0 1.0 0.0 null true))
  (bind _output_get (set `self.ActiveTheme` _returnvalue))
  (`AudioComponent.FadeIn` _output_get FadeInDuration 1.0 0.0 "Linear")
  (bind _returnvalue_2 (`|CreateWidget` "/Game/Blueprints/Menu/FadeMenu.FadeMenu_C"))
  (bind _output_get_2 (set `self.FadeInMenu` _returnvalue_2))
  (`UserWidget.AddToViewport` _output_get_2 6)
  (return (`self.FadeInMenu`)))

(fn `FadeOut`
  (params (FadeOutDuration :type "Float (single-precision)"))
  (returns (FadeInMenu :type "/Game/Blueprints/Menu/FadeMenu Object Reference"))
  (bind _activetheme (`self.ActiveTheme`))
  (`/Engine/EditorBlueprintResources/StandardMacros.IsValid` _activetheme
    (:`Is Valid`
      (`AudioComponent.FadeOut` _activetheme FadeOutDuration 0.0 "Linear"))
    (:`Is Not Valid`
      _))
  (bind _returnvalue (`|CreateWidget` "/Game/Blueprints/Menu/FadeMenu.FadeMenu_C"))
  (bind _output_get (set `self.FadeInMenu` _returnvalue))
  (`UserWidget.AddToViewport` _output_get 6)
  (return (`self.FadeInMenu`)))

(fn `SwitchMusic`
  (params (FadeDuration :type "Float (double-precision)") (Sound :type "SoundBase Object Reference"))
  (bind _activetheme (`self.ActiveTheme`))
  (`/Engine/EditorBlueprintResources/StandardMacros.IsValid` _activetheme
    (:`Is Valid`
      (`AudioComponent.FadeOut` _activetheme FadeDuration 0.0 "Linear"))
    (:`Is Not Valid`
      _))
  (bind _returnvalue (`GameplayStatics.CreateSound2D` Sound 1.0 1.0 0.0 null true))
  (bind _output_get (set `self.ActiveTheme` _returnvalue))
  (`AudioComponent.FadeIn` _output_get FadeDuration 1.0 0.0 "Linear")
  (return))

(fn `SwitchMusic+CreateFadeWidget_0`
  (params (FadeOutDuration :type "Float (double-precision)") (Sound :type "SoundBase Object Reference"))
  (returns (FadeInMenu :type "/Game/Blueprints/Menu/FadeMenu Object Reference"))
  (bind _activetheme (`self.ActiveTheme`))
  (`/Engine/EditorBlueprintResources/StandardMacros.IsValid` _activetheme
    (:`Is Valid`
      (`AudioComponent.FadeOut` _activetheme FadeOutDuration 0.0 "Linear")
      (bind _returnvalue (`|CreateWidget` "/Game/Blueprints/Menu/FadeMenu.FadeMenu_C"))
      (bind _output_get (set `self.FadeInMenu` _returnvalue))
      (`UserWidget.AddToViewport` _output_get 6)
      (`/Game/Blueprints/Menu/FadeMenu.FadeOut3` _output_get))
    (:`Is Not Valid`
      (bind _returnvalue_2 (`GameplayStatics.CreateSound2D` Sound 1.0 1.0 0.0 null true))
      (bind _output_get_2 (set `self.ActiveTheme` _returnvalue_2))
      (`AudioComponent.FadeIn` _output_get_2 FadeOutDuration 1.0 0.0 "Linear")
      (bind _returnvalue_3 (`|CreateWidget` "/Game/Blueprints/Menu/FadeMenu.FadeMenu_C"))
      (bind _output_get_3 (set `self.FadeInMenu` _returnvalue_3))
      (`UserWidget.AddToViewport` _output_get_3 6)
      (return (`self.FadeInMenu`)))))